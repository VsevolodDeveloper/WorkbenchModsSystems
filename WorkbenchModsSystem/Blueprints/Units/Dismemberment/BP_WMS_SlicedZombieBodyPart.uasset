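; A severed zombie body part that can be grabbed, stabbed and used to hit characters before dissolving away.
; The dissolve timer pauses while held and restarts on release, ending in a material fade and destruction.
; Hard impacts damage HSCharBase actors or leave oriented blood decals on static surfaces, while stabs create wounds through UnitWounds.
; The owner's death reason decides whether physics-constrained backbone or gut meshes stay attached.
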(event `self.SkeletalMeshComponent.OnComponentHit`
  (params (HitComponent :type "PrimitiveComponent Object Reference") (OtherActor :type "Actor Object Reference") (OtherComp :type "PrimitiveComponent Object Reference") (NormalImpulse :type "Vector Structure") (Hit :type "HitResult Structure (by ref)"))
  (bind (_bblockinghit _binitialoverlap _time _distance _location _impactpoint _normal _impactnormal) (`GameplayStatics.BreakHitResult` Hit))
  ;[1 1 1] Hit
  (`|ExecutionSequence`
    (:`then_0`
      (if (> (`KismetMathLibrary.VSize` NormalImpulse) 1000.0)
        (if (`|EnumEquality` (`PrimitiveComponent.GetCollisionObjectType` OtherComp) "ECC_WorldStatic")
          (`/Engine/EditorBlueprintResources/StandardMacros.DoOnce` false :!label _label
            (:`Completed`
              (`self.SpawnDecal` _impactpoint _impactnormal)
              (`GameplayStatics.PlaySoundAtLocation` "/Game/Sound/Gore/Cue/part_drop_Cue.part_drop_Cue" _impactpoint (struct) 1.0 1.0 0.0 null null null)
              (`KismetSystemLibrary.Delay` 1.0)
              (goto _label :!via `Reset`))))))
    (:`then_1`
      (if (> (`KismetMathLibrary.VSize` NormalImpulse) 1000.0)
        (bind _ashschar_base (cast `HSCharBase` OtherActor))
        (`/Engine/EditorBlueprintResources/StandardMacros.DoOnce` false :!label _label_2
          (:`Completed`
            (`HSHitableInterface.Hit` _ashschar_base (make `DamageInfo` "None" (struct) 200.0 1.0) Hit)
            (`GameplayStatics.PlaySoundAtLocation` "/Game/Sound/Fist/Cue/fist_hit_flesh_Cue.fist_hit_flesh_Cue" (`.ImpactPoint` (`GameplayStatics.BreakHitResult` Hit)) (struct) 1.0 1.0 0.0 null null null)
            (`KismetSystemLibrary.Delay` 0.5)
            (goto _label_2 :!via `Reset`)))))))

(event `self.ReceiveBeginPlay`
  (`|ExecutionSequence`
    (:`then_0`
      (`GrabHandlerComponent.LinkAll` (`self.GrabHandler`))
      (`KismetSystemLibrary.Delay` 0.1)
      (`SkeletalMeshComponent.SetNotifyRigidBodyCollisionBelow` (`self.SkeletalMeshComponent`) true "pelvis" true)
      (`self.SetScalarParameterValueOnAllMaterials` "BloodCoverage" 1.0)
      ;[1 1 1] Set Dissolve Timer
      (if (== (`GrabHandlerComponent.GetGrabbedPointsNum` (`self.GrabHandler`)) 0)
        (`self.SetDissolveTimer`))
      ;[1 1 1] Enable Stab after delay
      (`KismetSystemLibrary.Delay` 0.2)
      (set `self.bCanStab` true))
    (:`then_1`
      (`KismetSystemLibrary.Delay` 0.0)
      (`self.ManageAdditionalMeshes`))))

(event `SetDissolveTimer`
  (bind _returnvalue (`KismetSystemLibrary.K2_SetTimerDelegate` (`|CreateDelegate` :!event `StartDissolve`) (`self.LifeTime`)))
  (set `self.TimerHandle_DissolveTimer` _returnvalue))

(event `self.HSStabHandler.OnExtract`
  (params (InDamageType :type "EDamageType Enum" :default "Idle") (BoneName :type Name) (Point :type "Vector Structure") (DirectionInversed :type "Vector Structure") (StabData :type "StabData Structure (by ref)"))
  (`KismetSystemLibrary.RetriggerableDelay` 0.5)
  (set `self.bCanStab` true))

(event `self.GrabHandler.OnSnapPointBeginInteraction`
  (params (SnapPoint :type "SnapPointComponent Object Reference") (Hand :type "EHand Enum" :default "VR_LeftHand"))
  ;[1 1 1] Reset Dissolve Timer
  (`KismetSystemLibrary.K2_ClearAndInvalidateTimerHandle` (`self.TimerHandle_DissolveTimer`)))

(event `self.GrabHandler.OnSnapPointEndInteraction`
  (params (SnapPoint :type "SnapPointComponent Object Reference") (Hand :type "EHand Enum" :default "VR_LeftHand"))
  ;[1 1 1] Start dissolve when Nobody holds this actor
  (if (== (`GrabHandlerComponent.GetGrabbedPointsNum` (`self.GrabHandler`)) 0)
    (`self.SetDissolveTimer`)))

(event `StartDissolve`
  (bind _grabhandler (`self.GrabHandler`))
  ;[1 0.6423 0.02061] Dissolve
  (`GrabHandlerComponent.ReleaseAll` _grabhandler)
  (`GrabHandlerComponent.SetAccessibilityAll` _grabhandler "Disabled")
  (bind (_direction _dissolveintensity) (`Timeline|Dissolve` :!via `PlayFromStart`) ; Dissolve
    (:`Update`
      (for _array_element (`self.K2_GetComponentsByClass` "/Script/Engine.SkeletalMeshComponent")
        (`MeshComponent.SetScalarParameterValueOnMaterials` _array_element "DissolveIntensity" _dissolveintensity)))
    (:`Finished`
      (`self.K2_DestroyActor`))))

(event `self.HSStabHandler.OnStab`
  (params (InDamageType :type "HSDamageEventStab Object Reference") (RuleID :type "Name (by ref)") (HitResult :type "HitResult Structure (by ref)") (BoneName :type Name))
  (bind _structout (setmembers `DamageInfo` :`StructRef` (`self.Damage`) :`Damage` (`HSDamageEventBase.Damage` InDamageType) :`LinearVelocity` (`HSDamageEventBase.Velocity` InDamageType) :`bIsBash` false :`DamageType` (`HSDamageEventStab.DamageType` InDamageType)))
  (bind _returnvalue (`KismetMathLibrary.Normal` (`.LinearVelocity` (break `DamageInfo` _structout))))
  (set `self.NormalizedVelocity` _returnvalue)
  (`HSActorWoundsComponent.MakeWound` (`self.UnitWounds`) HitResult (`self.Damage`) (`self.NormalizedVelocity`) (`KismetMathLibrary.Cross_VectorVector` (`KismetMathLibrary.Cross_VectorVector` _returnvalue (`SceneComponent.GetUpVector` (`self.SkeletalMeshComponent`))) (`self.NormalizedVelocity`))))

(fn `GetRandomDecal`
  (params (Decals :type "Array of MaterialInterface Object Reference"))
  (returns (Decal :type "MaterialInterface Object Reference"))
  (return (`|GetArrayItem` Decals (`KismetMathLibrary.RandomIntegerInRange` 0 (`KismetArrayLibrary.Array_LastIndex` Decals)))))

(fn `IsActorAlive`
  (returns (ReturnValue :type Boolean))
  (return false))

(fn `ManageAdditionalMeshes`
  (locals (Character :type "/Game/Blueprints/Units/ALS_BaseCharacter Object Reference"))
  (bind _returnvalue (`self.GetOwner`))
  (`/Engine/EditorBlueprintResources/StandardMacros.IsValid` _returnvalue
    (:`Is Valid`
      (bind _asals_base_character (cast `/Game/Blueprints/Units/ALS_BaseCharacter` _returnvalue))
      (set `local.Character` _asals_base_character)
      (`|ExecutionSequence`
        (:`then_0`
          ;[1 1 1] BackBone
          (if (== (`HSCharBase.GetDeadReason` (`local.Character`)) "PullHead")
            (`PrimitiveComponent.SetSimulatePhysics` (`self.Backbone`) true)
            (`PhysicsConstraintComponent.SetConstrainedComponents` (`self.BackbonePhysicsConstraint`) (`self.Backbone`) "root_backbone" (`self.SkeletalMeshComponent`) "head")
            (`PhysicsConstraintComponent.SetConstraintReferenceFrame` (`self.BackbonePhysicsConstraint`) "Frame1" (`KismetMathLibrary.MakeTransform` (0.0 0.0 0.0)))
            (else
              (`ActorComponent.K2_DestroyComponent` (`self.Backbone`))
              (`ActorComponent.K2_DestroyComponent` (`self.BackbonePhysicsConstraint`)))))
        (:`then_1`
          ;[1 1 1] Gut
          (if (== (`HSCharBase.GetDeadReason` (`local.Character`)) "PelvisCut")
            (`PrimitiveComponent.SetSimulatePhysics` (`self.LowerGut`) true)
            (`PhysicsConstraintComponent.SetConstrainedComponents` (`self.LowerGutPhysicsConstraint`) (`self.LowerGut`) "guts_down_root" (`self.SkeletalMeshComponent`) "spine_01")
            (`PhysicsConstraintComponent.SetConstraintReferenceFrame` (`self.LowerGutPhysicsConstraint`) "Frame1" (`KismetMathLibrary.MakeTransform` (0.0 0.0 0.0)))
            (else
              (`ActorComponent.K2_DestroyComponent` (`self.LowerGut`))
              (`ActorComponent.K2_DestroyComponent` (`self.LowerGutPhysicsConstraint`)))))))))

(fn `SpawnDecal`
  (params (HitLocation :type "Vector Structure") (ImpactNormal :type "Vector Structure"))
  (if (> (`KismetMathLibrary.Dot_VectorVector` ImpactNormal (`KismetMathLibrary.MakeVector` 0.0 0.0 1.0)) (`self.SurfaceTypeDotTreshold`))
    ;[1 1 1] Horizontal
    (bind _decal (`self.GetRandomDecal` (`self.HorizontalDecals`)))
    (`/Engine/EditorBlueprintResources/StandardMacros.IsValid` _decal
      (:`Is Valid`
        (`|SpawnActorFromClass` "/Game/Blueprints/Decals/BP_BloodSplash.BP_BloodSplash_C" (`KismetMathLibrary.MakeTransform` (`local.HitLocation`) (`KismetMathLibrary.MakeRotFromXZ` (`KismetMathLibrary.RotateAngleAxis` (`KismetMathLibrary.Cross_VectorVector` (`KismetMathLibrary.MakeVector` 1.0) (`local.ImpactNormal`)) (`KismetMathLibrary.RandomFloatInRange` 0.0 360.0) (`local.ImpactNormal`)) (`local.ImpactNormal`))) "Undefined" "OverrideRootScale" null _decal null)))
    (else
      ;[1 1 1] Vertical
      (bind _decal_2 (`self.GetRandomDecal` (`self.VerticalDecals`)))
      (`/Engine/EditorBlueprintResources/StandardMacros.IsValid` _decal_2
        (:`Is Valid`
          (`|SpawnActorFromClass` "/Game/Blueprints/Decals/BP_BloodSplash.BP_BloodSplash_C" (`KismetMathLibrary.MakeTransform` (`local.HitLocation`) (`KismetMathLibrary.MakeRotFromXZ` (`KismetMathLibrary.Cross_VectorVector` (`local.ImpactNormal`) (`KismetMathLibrary.MakeVector` 0.0 0.0 1.0)) (`local.ImpactNormal`))) "Undefined" "OverrideRootScale" null _decal_2 null)))))
  (return))

(fn `TakeDamage`
  (params (DamageEvent :type "HSDamageEventBase Object Reference"))
  (returns (ReturnValue :type "HSDamageEventResult Structure"))
  (bind _hitresult (`HSDamageEventBase.HitResult` DamageEvent))
  (bind _ashsdamage_event_stab (cast `HSDamageEventStab` DamageEvent))
  (if (`self.bCanStab`)
    (bind (_outrule _returnvalue) (`HSStabHandlerComponent.K2_CanStab` (`self.HSStabHandler`) _ashsdamage_event_stab _hitresult (`.HitBoneName` (`GameplayStatics.BreakHitResult` _hitresult))))
    (if _returnvalue
      (set `self.bCanStab` false))
    (return (make `HSDamageEventResult` 0.0 true (make `HSStabResponse` _returnvalue)))))

(fn `UserConstructionScript`
  (`parent.UserConstructionScript`))