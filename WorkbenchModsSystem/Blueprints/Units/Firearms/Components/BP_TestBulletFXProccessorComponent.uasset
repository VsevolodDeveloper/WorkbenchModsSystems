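; Test bullet FX processor component that handles the flying sound of a bullet.
; On BeginPlay it caches its owner as an HSBulletBase.
; On the first Tick a DoOnce plays the bullet fly cue at player 0's pawn location, without a distance check.
; IsInPlayerRadius compares the bullet's distance to the player camera manager against CloseDistance, but the event graph never calls it.
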(event `self.ReceiveBeginPlay`
  (`parent.ReceiveBeginPlay`)
  (bind _ashsbullet_base (cast `HSBulletBase` (`self.GetOwner`)))
  (set `self.OwnerBullet` _ashsbullet_base))

(event `self.ReceiveTick`
  (params (DeltaSeconds :type "Float (single-precision)"))
  (`parent.ReceiveTick` DeltaSeconds)
  (`/Engine/EditorBlueprintResources/StandardMacros.DoOnce` false
    (:`Completed`
      (`GameplayStatics.PlaySoundAtLocation` "/Game/WorkbenchModsSystem/Sounds/Firearms/m_bullet_fly_Cue.m_bullet_fly_Cue" (`Actor.K2_GetActorLocation` (`GameplayStatics.GetPlayerPawn` 0)) (struct) 1.0 1.0 0.0 null null null))))

(fn `IsInPlayerRadius`
  (returns (ReturnValue :type Boolean))
  (bind _ownerbullet (`self.OwnerBullet`)
    (:`then`
      (return (<= (`Actor.GetDistanceTo` _ownerbullet (`GameplayStatics.GetPlayerCameraManager` 0)) (`self.CloseDistance`))))
    (:`else`)))