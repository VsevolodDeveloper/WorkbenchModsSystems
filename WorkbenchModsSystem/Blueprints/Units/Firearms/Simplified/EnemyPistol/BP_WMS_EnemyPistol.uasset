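; Simplified semi-automatic enemy pistol that wires trigger, hammer, barrel, slide, slide stop and magazine slot components into a firing cycle.
; The trigger strikes the hammer to fire the barrel; the shot pushes back the slide, which cocks the hammer and chambers live cartridges on return.
; Ammo state drives slide-stop lockup, last-shot sound and contextual Beretta M9 actions to release the slide or eject the magazine, briefly delayed after running empty.
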(event `self.ReceiveBeginPlay`
  ;[1 1 1] Initialization
  (`parent.ReceiveBeginPlay`)
  (`HSFirearmHTConstraintComponent.Initialize` (`self.TriggerHammerConstraint`) (`self.Hammer`) (`self.Trigger`) null)
  (set `HSAutomaticFirearmBoltComponent.IsLockedCallback` (`|CreateDelegate` :!event `ShutterIsLocked`) (`self.Slide`))
  (set `HSGunBarrelComponent.GetShotSoundCallback` (`|CreateDelegate` :!event `GetShotSound`) (`self.BarrelComponent`))
  (set `HSFirearmDATriggerComponent.OnCanPressTrigger` (`|CreateDelegate` :!event `CanPressTrigger`) (`self.Trigger`)))

(event `self.MagazineSlot.OnComponentMounted`
  (params (Slot :type "MountSlotComponent Object Reference") (MountedActor :type "Actor Object Reference") (MountedPrimitive :type "PrimitiveComponent Object Reference") (MountableComponent :type "MountableComponent Object Reference"))
  ;[1 1 1] Sets reference to the magazine when it has been mounted
  (bind _ashsfirearm_magazine_base (cast `HSFirearmMagazineBase` MountedActor))
  (bind _output_get (set `self.Magazine` _ashsfirearm_magazine_base))
  (`self.SetActorEnableCollision` _output_get false)
  (set `self.bCanRemoveMagazine` true))

(event `self.Trigger.OnTriggerPressed`
  (params (Trigger :type "HSFirearmTriggerComponentBase Object Reference"))
  ;[1 1 1] Activate the hammer to perform a strike
  (`HSFirearmHammerComponent.Strike` (`self.Hammer`)))

(event `self.Hammer.OnHit`
  (params (Hammer :type "HSFirearmHammerComponent Object Reference"))
  ;[1 1 1] Just shoot!
  (`HSGunBarrelComponent.Shot` (`self.BarrelComponent`)))

(event `self.Slide.OnMovedFromInitialPosition`
  (params (Bolt :type "HSFirearmBoltComponentBase Object Reference") (Ammo :type "Actor Object Reference"))
  ;[1 1 1] Clear the barrel's reference to the bullet when it moves out from initial position
  (`HSGunBarrelComponent.RemoveCartridge` (`self.BarrelComponent`)))

(event `self.Slide.OnActuated`
  (params (Bolt :type "HSFirearmBoltComponentBase Object Reference"))
  ;[1 1 1] Automatically cock the hammer when the shutter reaches particular position (ActuationRatio parameter)
  ; This is how semiauto handguns work, you don't need to cock a hammer manually, a shutter does it instead.
  (`|ExecutionSequence`
    (:`then_0`
      (bind _bshouldmoveup (`self.ShouldUpSlideStop`))
      (if _bshouldmoveup
        ;[1 1 1] If the player is out of Ammo, move the slide stop to up position and lock the shutter.
        ; There is also a one little trick when you have no ammo. We don't allow a player to extract the magazine immediately, but add a delay the player can press the trigger without making shot to allow time for making decisions about next actions
        (`HSWeaponSlideStopComponent.Up` (`self.SlideStop`))
        (set `self.bCanRemoveMagazine` false)
        (`KismetSystemLibrary.K2_SetTimerDelegate` (delegate `CanRemoveMagazine`) 1.0)))
    (:`then_1`
      (`HSFirearmHammerComponent.Cock` (`self.Hammer`) 20.0))))

(event `CanRemoveMagazine`
  ;[1 1 1] If the player is out of Ammo, move the slide stop to up position and lock the shutter.
  ; There is also a one little trick when you have no ammo. We don't allow a player to extract the magazine immediately, but add a delay the player can press the trigger without making shot to allow time for making decisions about next actions
  (set `self.bCanRemoveMagazine` true))

(event `self.Slide.OnMovedToInitialPosition`
  (params (Bolt :type "HSFirearmBoltComponentBase Object Reference") (Ammo :type "Actor Object Reference"))
  ;[1 1 1] Updates a cartridge in the barrel is the first one is not a shell. It's necessary to a barrel knows about the cartridge to make a shot
  (bind _ashsfirearm_cartridge_interface (cast `HSFirearmCartridgeInterface` Ammo))
  (if (not (`HSFirearmCartridgeInterface.IsShell` _ashsfirearm_cartridge_interface))
    (`HSGunBarrelComponent.SetCartridge` (`self.BarrelComponent`) _ashsfirearm_cartridge_interface)))

(event `self.BarrelComponent.OnShot`
  (params (Barrel :type "HSGunBarrelComponent Object Reference") (Cartridge :type "HSFirearmCartridgeInterface Interface (by ref)") (Bullets :type "Array of Actor Object Reference (by ref)"))
  ;[1 1 1] Called immediately after shot, we need to push back the slide because of powder gases
  ; Parallely we play muzzle FX and add the weapon recoil
  (`self.PlayMuzzleEffects`)
  (`HSAutomaticFirearmBoltComponent.PushBack` (`self.Slide`)))

(event `self.Trigger.OnActionRequested`
  (params (Trigger :type "HSFirearmTriggerComponentBase Object Reference") (SnapPoint :type "SnapPointComponent Object Reference"))
  (bind _returnvalue (`ElasticVRFunctionLibrary.GetFirstGrabbingMotionController` SnapPoint))
  ;[1 1 1] Called on custom action request
  (`self.GetAmmoState`
    (:`NoMagazine`
      (if (`HSWeaponSlideStopComponent.IsUp` (`self.SlideStop`)) :!label _label
        ;[1 1 1] If we have an ammo or don't have loaded magazine and but slide stop is up, then move slide stop down and unlock the shutter
        (`|PerformSPAdditionalAction` SnapPoint _returnvalue "/Game/Blueprints/Weapons/Firearms/Actions/BP_BerettaM9_MoveSlideStopDownAction.BP_BerettaM9_MoveSlideStopDownAction_C"
          (:`then`
            (`/Engine/EditorBlueprintResources/StandardMacros.DoOnce` false :!label _label_2
              (:`Completed`
                (`KismetSystemLibrary.Delay` 0.4)
                (bind _returnvalue_2 (`HSWeaponSlideStopComponent.Down` (`self.SlideStop`)))
                (if _returnvalue_2
                  (`HSAutomaticFirearmBoltComponent.Unlock` (`self.Slide`))))))
          (:`OnFinished`
            (goto _label_2 :!via `Reset`)))))
    (:`HasAmmo`
      (goto _label))
    (:`NoAmmo`
      ;[1 1 1] If there is no ammo, dismount the magazine
      (`|PerformSPAdditionalAction` SnapPoint _returnvalue "/Game/Blueprints/Weapons/Firearms/Actions/BP_BerettaM9_UnmountMagazineAction.BP_BerettaM9_UnmountMagazineAction_C"
        (:`then`
          (`/Engine/EditorBlueprintResources/StandardMacros.DoOnce` false :!label _label_3
            (:`Completed`
              (`KismetSystemLibrary.Delay` 0.2)
              (`MountSlotComponent.Dismount` (`self.MagazineSlot`) false))))
        (:`OnFinished`
          (goto _label_3 :!via `Reset`))))))

(event `self.MagazineSlot.OnComponentDismounted`
  (params (Slot :type "MountSlotComponent Object Reference") (MountedActor :type "Actor Object Reference") (MountedPrimitive :type "PrimitiveComponent Object Reference") (MountableComponent :type "MountableComponent Object Reference"))
  ;[1 1 1] If there is no ammo, dismount the magazine
  (set `self.Magazine` null))

(fn `CanPressTrigger`
  (returns (ReturnValue :type Boolean))
  (bind _returnvalue (`HSWeaponSlideStopComponent.IsDown` (`self.SlideStop`)))
  (`self.GetAmmoState`
    (:`NoMagazine`
      (return _returnvalue))
    (:`HasAmmo`
      (return _returnvalue))
    (:`NoAmmo`
      (return (or (`HSGunBarrelComponent.IsLoaded` (`self.BarrelComponent`)) (== (`self.bCanRemoveMagazine`) false))))))

(fn `GetShotSound`
  (params (ReferenceSound :type "SoundBase Object Reference") (Caliber :type "GameplayTag Structure (by ref)"))
  (returns (ReturnValue :type "SoundBase Object Reference"))
  (bind _magazine (`self.Magazine`)
    (:`then`
      (return (select `bool` (`HSFirearmMagazineBase.IsAmmoLeft` _magazine) :`false` (`self.LastShotSound`) :`true` (`local.ReferenceSound`))))
    (:`else`
      (return (`self.LastShotSound`)))))

(fn `PlayMuzzleEffects`
  (`ActorComponent.Activate` (`self.MuzzleParticles`) true))

(fn `ShouldUpSlideStop`
  (returns (bShouldMoveUp :type Boolean))
  (`self.GetAmmoState`
    (:`NoMagazine`
      (return (`HSAutomaticFirearmBoltComponent.IsMovedByPowderGases` (`self.Slide`))))
    (:`HasAmmo`
      (return false))
    (:`NoAmmo`
      (return true))))

(fn `ShutterIsLocked`
  (returns (ReturnValue :type Boolean))
  (return false))

(fn `UserConstructionScript`)