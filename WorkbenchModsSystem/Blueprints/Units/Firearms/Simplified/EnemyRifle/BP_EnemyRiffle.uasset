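; Simplified enemy rifle Blueprint that fires single, automatic or burst shots.
; Trigger presses fire the barrel, which pushes back the shutter and plays muzzle particles; the returning shutter chambers live cartridges and refires in automatic mode while the trigger is held.
; A mounted magazine is stored with its collision disabled.
; The Shot event repeats the parent shot a random number of times with a short delay, producing sprays.
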(event `self.Trigger.OnTriggerPressed`
  (params (Trigger :type "HSFirearmTriggerComponentBase Object Reference"))
  ;[1 1 1] Activate the hammer to perform a strike
  (`HSGunBarrelComponent.Shot` (`self.BarrelComponent`)))

(event `self.BarrelComponent.OnShot`
  (params (Barrel :type "HSGunBarrelComponent Object Reference") (Cartridge :type "HSFirearmCartridgeInterface Interface (by ref)") (Bullets :type "Array of Actor Object Reference (by ref)"))
  ;[1 1 1] Called immediately after shot, we need to push back the shutter because of powder gases. Parallely we play muzzle FX and add the weapon recoil
  (`HSAutomaticFirearmBoltComponent.PushBack` (`self.Shutter`))
  (`ActorComponent.Activate` (`self.MuzzleParticles`) false))

(event `self.Trigger.OnTriggerReleased`
  (params (Trigger :type "HSFirearmTriggerComponentBase Object Reference"))
  ;[1 1 1] Deactive muzzle particles when trigger is released
  (`ActorComponent.Deactivate` (`self.MuzzleParticles`)))

(event `self.Shutter.OnMovedFromInitialPosition`
  (params (Bolt :type "HSFirearmBoltComponentBase Object Reference") (Ammo :type "Actor Object Reference"))
  ;[1 1 1] Clear the barrel's reference to the bullet when it moves out from initial position
  (`HSGunBarrelComponent.RemoveCartridge` (`self.BarrelComponent`)))

(event `self.MagazineSlot.OnComponentMounted`
  (params (Slot :type "MountSlotComponent Object Reference") (MountedActor :type "Actor Object Reference") (MountedPrimitive :type "PrimitiveComponent Object Reference") (MountableComponent :type "MountableComponent Object Reference"))
  ;[0.978 1 0.4595] Called when a magazine is mounted
  (bind _ashsfirearm_magazine_base (cast `HSFirearmMagazineBase` (`ActorComponent.GetOwner` MountedPrimitive)))
  (bind _output_get (set `self.Magazine` _ashsfirearm_magazine_base))
  (`self.SetActorEnableCollision` _output_get false))

(event `self.Shutter.OnMovedToInitialPosition`
  (params (Bolt :type "HSFirearmBoltComponentBase Object Reference") (Ammo :type "Actor Object Reference"))
  ;[1 1 1] Updates a cartridge in the barrel is the first one is not a shell. It's necessary to a barrel knows about the cartridge to make a shot
  (bind _ashsfirearm_cartridge_interface (cast `HSFirearmCartridgeInterface` Ammo)
    (:`then`
      (if (not (`HSFirearmCartridgeInterface.IsShell` _ashsfirearm_cartridge_interface))
        (`HSGunBarrelComponent.SetCartridge` (`self.BarrelComponent`) _ashsfirearm_cartridge_interface)
        ;[1 1 1] If the trigger is pressed, then automatically shoot
        (if (and (`HSFirearmTriggerComponentBase.IsPressed` (`self.Trigger`)) (`self.bAutomaticMode`))
          (`HSGunBarrelComponent.Shot` (`self.BarrelComponent`))
          (else
            (`ActorComponent.Deactivate` (`self.MuzzleParticles`) :!label _label)))
        (else
          (goto _label))))
    (:`CastFailed`
      (goto _label))))

(event `self.Shot`
  ;[1 1 1] Shot!
  (`/Game/Blueprints/Helpers/HSActorsMacroLibrary.ForLoopWithDelay` 0 (`KismetMathLibrary.RandomIntegerInRange` (`self.MinShotsInOneSpray`) (`self.MaxShotsInOneSpray`)) 0.1 0.1
    (:`LoopBody`
      (`parent.Shot`))))

(fn `UserConstructionScript`)