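; Base firearm for enemy units: fires cartridges from its magazine through a gun barrel component and supplies randomized moveset animations.
; Each tick, it can aim the barrel at Target with random spread, independently of the mesh.
; Reloading blocks shots while the magazine is dismounted, a replacement spawns on a mesh socket and is remounted to the cached slot.
; In constrained mode, a physics constraint locks or frees the owner's left hand on the weapon.
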(event `self.ReceiveBeginPlay`
  (`parent.ReceiveBeginPlay`)
  (`self.Initialize`))

(event `self.ReceiveTick`
  (params (DeltaSeconds :type "Float (single-precision)"))
  (`parent.ReceiveTick` DeltaSeconds)
  (`self.RotateBarrelToTarget`))

(fn `AddWeaponOffset`
  (`self.K2_AddActorLocalTransform` (`self.WeaponOffset`)))

(fn `AmmoIsOut`
  (returns (ReturnValue :type Boolean))
  (bind _magazine (`self.Magazine`)
    (:`then`
      (return (== (`HSFirearmMagazineBase.AmmoNum` _magazine) 0)))
    (:`else`
      (bind _stackmagazine (`self.StackMagazine`)
        (:`then`
          (return (`HSActorsStackComponent.IsEmpty` _stackmagazine)))
        (:`else`)))))

(fn `AttachMagazine`
  (bind _cachedmagazine (`self.CachedMagazine`)
    (:`then`
      (`self.K2_DetachFromActor` _cachedmagazine "KeepWorld" "KeepWorld" "KeepRelative")
      (`self.K2_AttachToComponent` (`self.CachedMagazine`) (`self.CachedMountSlot`) "None" "SnapToTarget" "SnapToTarget" "KeepRelative" true))
    (:`else`)))

(fn `DismountMagazine`
  (bind _magazine (`self.Magazine`)
    (:`then`
      (bind _returnvalue (`MountableComponent.GetSlotMountedTo` (`HSFirearmMagazineBase.MountableComp` _magazine)))
      (`/Engine/EditorBlueprintResources/StandardMacros.IsValid` _returnvalue
        (:`Is Valid`
          (bind _output_get (set `self.CachedMountSlot` _returnvalue))
          (`MountSlotComponent.Dismount` _output_get true))))
    (:`else`)))

(fn `FinishReload`
  (set `self.bReloading` false)
  (set `self.Magazine` (`self.CachedMagazine`))
  (bind _cachedmountslot (`self.CachedMountSlot`)
    (:`then`
      (bind _magazine (`self.Magazine`)
        (:`then`
          (`MountableComponent.MountToSlot` (`HSFirearmMagazineBase.MountableComp` _magazine) _cachedmountslot true false))
        (:`else`)))
    (:`else`)))

(fn `GetAmmo`
  (returns (Ammo :type "HSFirearmCartridgeInterface Interface"))
  (bind _magazine (`self.Magazine`)
    (:`then`
      (bind _ammo (`HSFirearmMagazineBase.TakeAmmo` _magazine))
      (return _ammo))
    (:`else`)))

(fn `GetMovesetAnimations`
  (returns (AimAnimation :type "AnimSequence Object Reference") (IdleCombatAnimation :type "AnimSequence Object Reference") (IdleCalmAnimation :type "AnimSequence Object Reference") (IdleCrouchAnimation :type "AnimSequence Object Reference") (AimCrouchAnimation :type "AnimSequence Object Reference") (AimOffset :type "AimOffsetBlendSpace Object Reference"))
  (return (`KismetArrayLibrary.Array_Random` (`self.AimAnimations`)) (`KismetArrayLibrary.Array_Random` (`self.IdleCombatAnimations`)) (`KismetArrayLibrary.Array_Random` (`self.IdleCalmAnimations`)) (`KismetArrayLibrary.Array_Random` (`self.IdleCrouchAnimations`)) (`KismetArrayLibrary.Array_Random` (`self.AimCrouchAnimations`)) (`self.AimOffset`)))

(fn `Initialize`
  (bind _returnvalue (`HSCommonFunctionLibrary.GetComponentByName` self "MagazineComponent"))
  (set `self.Barrel` (`self.GetComponentByClass` "/Script/Hellsplit_Arena.HSGunBarrelComponent"))
  (`/Engine/EditorBlueprintResources/StandardMacros.IsValid` _returnvalue
    (:`Is Valid`
      (bind _asfirearm_magazine (cast `HSFirearmMagazineComponent` _returnvalue))
      (set `self.StackMagazine` _asfirearm_magazine))))

(fn `LinkHands`
  (params (LeftHandConstraint :type "PhysicsConstraintComponent Object Reference"))
  (if (`self.bConstrainedMode`)
    (`ElasticVRFunctionLibrary.UpdateComponentTransform` (`self.MeshComp`))
    (`PhysicsConstraintComponent.SetLinearXLimit` (`local.LeftHandConstraint`) "LCM_Locked" 0.0)
    (`PhysicsConstraintComponent.SetLinearYLimit` (`local.LeftHandConstraint`) "LCM_Locked" 0.0)
    (`PhysicsConstraintComponent.SetLinearZLimit` (`local.LeftHandConstraint`) "LCM_Locked" 0.0)
    (`PhysicsConstraintComponent.SetAngularSwing1Limit` (`local.LeftHandConstraint`) "ACM_Locked" 0.0)
    (`PhysicsConstraintComponent.SetAngularSwing2Limit` (`local.LeftHandConstraint`) "ACM_Locked" 0.0)
    (`PhysicsConstraintComponent.SetAngularTwistLimit` (`local.LeftHandConstraint`) "ACM_Locked" 0.0)))

(fn `RotateBarrelToTarget`
  (bind _returnvalue (`KismetMathLibrary.RandomFloatInRange` 0.0 (`self.MaxSpreadAngle`)))
  (bind _target (`self.Target`)
    (:`then`
      (if (`self.bRotateBarrelToTarget`)
        (bind _barrel (`self.Barrel`)
          (:`then`
            (`SceneComponent.K2_SetWorldRotation` _barrel (`HSCommonFunctionLibrary.AddDeltaRotation` (`KismetMathLibrary.FindLookAtRotation` (`SceneComponent.K2_GetComponentLocation` (`self.Barrel`)) (`self.K2_GetActorLocation` _target)) (`KismetMathLibrary.MakeRotator` _returnvalue _returnvalue _returnvalue)) false false))
          (:`else`))))
    (:`else`)))

(fn `SetTwoHandedMode`
  (params (OwnerMesh :type "SkeletalMeshComponent Object Reference") (LeftHandConstraint :type "PhysicsConstraintComponent Object Reference"))
  (bind (_returnvalue_location _returnvalue_rotation) (`KismetMathLibrary.BreakTransform` (`SceneComponent.GetSocketTransform` (`self.MeshComp`) "hand_l" "RTS_Component")))
  (`/Engine/EditorBlueprintResources/StandardMacros.IsValid` OwnerMesh
    (:`Is Valid`
      (if (`self.bConstrainedMode`)
        (`ElasticVRFunctionLibrary.UpdateComponentTransform` (`self.MeshComp`))
        (`PhysicsConstraintComponent.SetConstrainedComponents` (`local.LeftHandConstraint`) (`local.OwnerMesh`) "hand_l" (`self.MeshComp`) "hand_l")
        (`PhysicsConstraintComponent.SetConstraintReferenceFrame` (`local.LeftHandConstraint`) "Frame2" (`KismetMathLibrary.MakeTransform` _returnvalue_location _returnvalue_rotation))))))

(fn `Shot`
  (if (not (`self.bReloading`))
    (bind _ammo (`self.GetAmmo`))
    (bind _barrel (`self.Barrel`)
      (:`then`
        (`HSGunBarrelComponent.SetCartridge` _barrel _ammo)
        (`HSGunBarrelComponent.Shot` (`self.Barrel`)))
      (:`else`))))

(fn `SpawnMagazine`
  (params (Mesh :type "SkeletalMeshComponent Object Reference"))
  (bind _returnvalue (`|SpawnActorFromClass` (`self.MagazineClass`) (`SceneComponent.GetSocketTransform` (`local.Mesh`) "socket_bow" "RTS_World") "AlwaysSpawn" "OverrideRootScale" null null))
  (set `self.CachedMagazine` _returnvalue)
  (bind _cachedmagazine (`self.CachedMagazine`)
    (:`then`
      (`SceneComponent.K2_AttachToComponent` (`HSFirearmMagazineBase.MeshComp` _cachedmagazine) (`local.Mesh`) "socket_bow" "SnapToTarget" "SnapToTarget" "KeepRelative" true))
    (:`else`)))

(fn `StartToReload`
  (set `self.bReloading` true)
  (`self.DismountMagazine`)
  (set `self.Magazine` null))

(fn `UnlinkHands`
  (params (LeftHandConstraint :type "PhysicsConstraintComponent Object Reference"))
  (if (`self.bConstrainedMode`)
    (`ElasticVRFunctionLibrary.UpdateComponentTransform` (`self.MeshComp`))
    (`PhysicsConstraintComponent.SetLinearXLimit` (`local.LeftHandConstraint`) "LCM_Free" 0.0)
    (`PhysicsConstraintComponent.SetLinearYLimit` (`local.LeftHandConstraint`) "LCM_Free" 0.0)
    (`PhysicsConstraintComponent.SetLinearZLimit` (`local.LeftHandConstraint`) "LCM_Free" 0.0)
    (`PhysicsConstraintComponent.SetAngularSwing1Limit` (`local.LeftHandConstraint`) "ACM_Free" 0.0)
    (`PhysicsConstraintComponent.SetAngularSwing2Limit` (`local.LeftHandConstraint`) "ACM_Free" 0.0)
    (`PhysicsConstraintComponent.SetAngularTwistLimit` (`local.LeftHandConstraint`) "ACM_Free" 0.0)))

(fn `UserConstructionScript`
  (`parent.UserConstructionScript`))