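; BP_WMS_AmbientController switches an AmbientSound object between ambient and battle music based on round state and player mounting.
; After a short startup delay, it binds to BP_HSGameMode round events and player avatar mount events, then starts the default ambient song.
; Round events only set a RoundStart flag.
; While that flag is set, dismounting plays the battle song and mounting returns to ambient.
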(event `self.ReceiveBeginPlay`
  (bind _ambientsound (`self.AmbientSound`))
  (`KismetSystemLibrary.Delay` 0.1) ; Wait for initialize
  (`self.SetupGameModeReference`)
  (`self.SetupBindings`)
  (`/Engine/EditorBlueprintResources/StandardMacros.IsValid` _ambientsound
    (:`Is Valid`
      (`AudioComponent.SetSound` (`AmbientSound.AudioComponent` _ambientsound) (`self.DefaultAmbientSound`))
      (`/Game/Blueprints/Common/BP_AmbientSound.DoAmbientSong` _ambientsound))))

(fn `OnDismount`
  (params (ControlledActor :type "Actor Object Reference"))
  (`self.PlayBattleSound`))

(fn `OnMount`
  (params (ControlledActor :type "Actor Object Reference"))
  (`self.StopBattleSound`))

(fn `OnRoundEnd`
  (params (RoundStats :type "HSRoundStatsCollector Object Reference"))
  (set `self.bRoundStart` false))

(fn `OnRoundStart`
  (locals (PlayerAvatar :type "HSPlayerAvatar Object Reference"))
  (set `self.bRoundStart` true))

(fn `PlayBattleSound`
  (locals (ActionAudio :type "AudioComponent Object Reference"))
  (if (and (`KismetSystemLibrary.IsValid` (`self.AmbientSound`)) (`self.bRoundStart`))
    (`/Game/Blueprints/Common/BP_AmbientSound.DoBattleSong` (`self.AmbientSound`) false)))

(fn `SetupBindings`
  (locals (PlayerAvatar :type "HSPlayerAvatar Object Reference"))
  (bind _output_get (set `local.PlayerAvatar` (`HSPlayerFunctionLibrary.GetPlayerAvatar`)))
  (`/Engine/EditorBlueprintResources/StandardMacros.IsValid` _output_get
    (:`Is Valid`
      (add `HSVRCharacter.OnMount` (`local.PlayerAvatar`) (`|CreateDelegate` :!event `OnMount`))
      (add `HSVRCharacter.OnDismount` (`local.PlayerAvatar`) (`|CreateDelegate` :!event `OnDismount`)))))

(fn `SetupGameModeReference`
  (bind _output_get (set `self.GameMode` (cast `/Game/Blueprints/General/BP_HSGameMode` (`GameplayStatics.GetGameMode`) :!pure true)))
  (`/Engine/EditorBlueprintResources/StandardMacros.IsValid` _output_get
    (:`Is Valid`
      (add `Hellsplit_ArenaGameModeBase.OnRoundBegun` (`self.GameMode`) (`|CreateDelegate` :!event `OnRoundStart`))
      (add `Hellsplit_ArenaGameModeBase.OnRoundEnd` (`self.GameMode`) (`|CreateDelegate` :!event `OnRoundEnd`)))))

(fn `StopBattleSound`
  (locals (ActionAudio :type "AudioComponent Object Reference"))
  (if (and (`KismetSystemLibrary.IsValid` (`self.AmbientSound`)) (`self.bRoundStart`))
    (`/Game/Blueprints/Common/BP_AmbientSound.DoAmbientSong` (`self.AmbientSound`))))

(fn `UserConstructionScript`)