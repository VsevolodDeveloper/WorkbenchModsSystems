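; BP_WMS_MusicSystem is a music system actor that maps named configs to sets of sounds.
; On BeginPlay it spawns the AudioTemplate actor and initializes it with its audio component, itself and a fade duration.
; Helpers pick a random sound for a config or reverse-lookup a sound's config by struct comparison.
; SetConfigsFromTemplate adds the template's default AvailableConfigs as map keys, pairing them with existing sound sets by index.
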(event `self.ReceiveBeginPlay`
  (bind _returnvalue (`|SpawnActorFromClass` (`self.AudioTemplate`) (`self.SpawnTransform`) "AlwaysSpawn" "OverrideRootScale" null null))
  (`/Game/WorkbenchModsSystem/Blueprints/Environment/MusicSystem/Templates/BP_WMS_MusicTemplateBase.Initialize` _returnvalue (`self.Audio`) self (`self.FadeDuration`)))

(fn `GetAudioByConfig`
  (params (Config :type Name))
  (returns (SelectedSound :type "SoundBase Object Reference"))
  (locals (Keys :type "Array of SoundBase Object Reference") (SelectedSounds :type "Set of SoundBase Object Reference"))
  (bind _result (`BlueprintSetLibrary.Set_ToArray` (`.Sounds_6_B34D0BAA484F5C0CA8FD9EA760BAD6F5` (break `/Game/WorkbenchModsSystem/Blueprints/Environment/MusicSystem/F_WMS_MusicConfiguration` (`BlueprintMapLibrary.Map_Find` (`self.SoundsByConfig`) Config)))))
  (return (`KismetArrayLibrary.Array_Random` _result)))

(fn `GetConfigByAudio`
  (params (Sound :type "SoundBase Object Reference"))
  (returns (Config :type Name))
  (locals (SelectedSounds :type "/Game/WorkbenchModsSystem/Blueprints/Environment/MusicSystem/F_WMS_MusicConfiguration Structure"))
  (bind _values (`BlueprintMapLibrary.Map_Values` (`self.SoundsByConfig`)))
  (for _array_element _values
    (bind _result (`BlueprintSetLibrary.Set_ToArray` (`.Sounds_6_B34D0BAA484F5C0CA8FD9EA760BAD6F5` (break `/Game/WorkbenchModsSystem/Blueprints/Environment/MusicSystem/F_WMS_MusicConfiguration` _array_element))))
    (if (`KismetArrayLibrary.Array_Contains` _result (`local.Sound`))
      (set `local.SelectedSounds` _array_element)))
  (bind _keys (`BlueprintMapLibrary.Map_Keys` (`self.SoundsByConfig`)))
  (for _array_element_2 _keys
    (if (`/Game/WorkbenchModsSystem/Blueprints/MacroLibrary/WMS_MacroLibrary.WMS_Equal(Structs)` (`BlueprintMapLibrary.Map_Find` (`self.SoundsByConfig`) _array_element_2) (`local.SelectedSounds`))
      (return _array_element_2)))
  (return "None"))

(fn `SetConfigsFromTemplate`
  (locals (Configs :type "Array of Name") (Sounds :type "Array of /Game/WorkbenchModsSystem/Blueprints/Environment/MusicSystem/F_WMS_MusicConfiguration Structure"))
  (bind _result (`BlueprintSetLibrary.Set_ToArray` (`.AvailableConfigs` (defaults `Object` (`self.AudioTemplate`)))))
  (set `local.Configs` _result)
  (bind _values (`BlueprintMapLibrary.Map_Values` (`self.SoundsByConfig`)))
  (set `local.Sounds` _values)
  (for (_array_element _array_index) (`local.Configs`)
    (`BlueprintMapLibrary.Map_Add` (`self.SoundsByConfig`) _array_element (`|GetArrayItem` (`local.Sounds`) _array_index))))

(fn `UserConstructionScript`)