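; BP_AdvancedSlotComponent is a placement component that spawns an equipment holder on its parent skeletal mesh at BeginPlay.
; It spawns the configured holder class at its transform plus an offset, passing haptics, radius, name, allowed classes and gameplay tags, with a separate branch for avatar weapon holders.
; The holder attaches to the configured socket keeping world transform and receives any initial equipment.
; The component clears its static mesh and destroys itself afterwards.
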(event `self.ReceiveBeginPlay`
  (`self.SpawnSlot`))

(fn `AddOffset`
  (params (WorldTransform :type "Transform Structure"))
  (returns (ReturnValue :type "Transform Structure"))
  (bind (_additionaltransform_location _additionaltransform_rotation) (`KismetMathLibrary.BreakTransform` (`self.AdditionalTransform`)))
  (return (`KismetMathLibrary.MakeTransform` (`KismetMathLibrary.TransformLocation` WorldTransform _additionaltransform_location) (`KismetMathLibrary.TransformRotation` WorldTransform _additionaltransform_rotation) (.scale WorldTransform))))

(fn `GetSpawnTransformOfSlot`
  (returns (ReturnValue :type "Transform Structure"))
  (return (`self.AddOffset` (`self.K2_GetComponentToWorld`))))

(fn `SpawnSlot`
  (locals (Mesh :type "SkeletalMeshComponent Object Reference"))
  (`|ExecutionSequence`
    (:`then_0`
      (`self.SetStaticMesh` null)
      (bind _asskeletal_mesh_component (cast `SkeletalMeshComponent` (`self.GetAttachParent`)))
      (set `local.Mesh` _asskeletal_mesh_component)
      (bind _asbp_avatar_weapon_holder (castclass `/Game/Blueprints/Player/Interactives/Holders/BP_AvatarWeaponHolder` (`self.Class`))
        (:`then`
          (bind _returnvalue (`|SpawnActorFromClass` _asbp_avatar_weapon_holder (`self.GetSpawnTransformOfSlot`) "AlwaysSpawn" "OverrideRootScale" null 0 (`self.GameplayTags`) (`self.HoldHapticEventId`) (`self.ReleaseHapticEventId`) (`self.SphereRadius`) (`self.HolderName`) (`self.AllowedClasses`) null))
          (bind _output_get (set `self.NewSlot` _returnvalue))
          (`Actor.K2_AttachToComponent` _output_get (`local.Mesh`) (`self.SocketName`) "KeepWorld" "KeepWorld" "KeepWorld" false))
        (:`CastFailed`
          (bind _returnvalue_2 (`|SpawnActorFromClass` (`self.Class`) (`self.GetSpawnTransformOfSlot`) "AlwaysSpawn" "OverrideRootScale" null (`self.HoldHapticEventId`) (`self.ReleaseHapticEventId`) (`self.SphereRadius`) (`self.HolderName`) (`self.AllowedClasses`) null))
          (bind _output_get_2 (set `self.NewSlot` _returnvalue_2))
          (message `/Game/WorkbenchModsSystem/Blueprints/Interfaces/BPI_WMS_SlotInterface.SetTags` _output_get_2 (`self.GameplayTags`))
          (`Actor.K2_AttachToComponent` (`self.NewSlot`) (`local.Mesh`) (`self.SocketName`) "KeepWorld" "KeepWorld" "KeepWorld" false))))
    (:`then_1`
      (if (`KismetSystemLibrary.IsValidClass` (`self.InitialEquipment`))
        (bind _returnvalue_3 (`|SpawnActorFromClass` (`self.InitialEquipment`) (`KismetMathLibrary.MakeTransform` (0.0 0.0 0.0)) "AlwaysSpawn" "OverrideRootScale" null null))
        (`HSHolderBase.PutActorToHolder` (`self.NewSlot`) _returnvalue_3)))
    (:`then_2`
      (`self.K2_DestroyComponent`))))