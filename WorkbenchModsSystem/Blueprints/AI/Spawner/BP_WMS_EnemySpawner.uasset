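; Wave spawner actor that spawns enemies by wave ID from presets loaded from a data table, through a shared unit factory.
; An initial chance-based burst uses preset-specific or random spawn points, consuming each point.
; Further ratio-weighted spawns follow on a delay driven by kill-progress curve, queuing when the alive cap is reached.
; Spawn and pre-death events track counts until the kill goal fires the completion event and disables the spawner.
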(event `self.ReceiveBeginPlay`
  (if (`KismetSystemLibrary.IsValidClass` (`self.UnitFactoryClass`))
    (bind _returnvalue (`GameplayStatics.GetActorOfClass` (`self.UnitFactoryClass`)))
    (`/Engine/EditorBlueprintResources/StandardMacros.IsValid` _returnvalue
      (:`Is Valid`
        (set `self.UnitFactory` _returnvalue))
      (:`Is Not Valid`
        (bind _returnvalue_2 (`|SpawnActorFromClass` (`self.UnitFactoryClass`) (`KismetMathLibrary.MakeTransform` (0.0 0.0 0.0)) "Undefined" "OverrideRootScale" null null))
        (set `self.UnitFactory` _returnvalue_2)))
    (else
      (`KismetSystemLibrary.PrintString` "UnitFactoryClass Is None" true true (struct :`R` 1.0 :`G` 0.192062 :`A` 1.0)))))

(event `OnUnitSpawned`
  (params (Unit :type "Actor Object Reference") (UnitPresetName :type Name) (Success :type Boolean))
  ;[1 1 1] OnUnitEvents
  (if Success
    (`/Engine/EditorBlueprintResources/StandardMacros.IncrementInt` (`self.EnemiesAlive`)
      (:`  `
        (bind _ashschar_base (cast `HSCharBase` Unit))
        (add `HSCharBase.OnPreDead` _ashschar_base (`|CreateDelegate` :!event `OnUnitDead`))
        (`self.DecrementSpawnAmount` UnitPresetName)
        (message `/Game/WorkbenchModsSystem/Blueprints/Interfaces/BPI_WMS_EnemyInterface.SpawnStartEffect` Unit)))))

(event `SpawnAtTheStart`
  (bind _cachedstartpoints (`self.CachedStartPoints`))
  ;[1 1 1] SpawnAtStart
  (set `self.CachedStartPoints` (`self.CachedAllPoints`))
  (`|ExecutionSequence`
    (:`then_0`
      (bind _element (`/Game/WorkbenchModsSystem/Blueprints/MacroLibrary/WMS_MacroLibrary.WMS_ForEachLoopWithBreakAndDelay` (`.EnemiesToSpawn_43_72F9EC6D4366F1317AC1069CF36B1151` (break `/Game/WorkbenchModsSystem/Blueprints/AI/Spawner/F_WMS_EnemySpawnerSettings` (`self.CachedEnemySpawnerSettings`))) (`self.StartSpawnAsyncTime`) :!label _label)
        (:`Loop Body`
          (bind ((`MaxToSpawnAtStart_18_B87C6E9E4D816F37C059F6A5192AE7D5` _maxtospawnatstart) (`MaxToSpawn_19_63846AB7475BF2D8B145BCA912440D96` _maxtospawn)) (break `/Game/WorkbenchModsSystem/Blueprints/AI/Spawner/F_WMS_EnemySettings` _element))
          (bind _returnvalue (`KismetMathLibrary.Min` _maxtospawnatstart _maxtospawn))
          (if (!= _returnvalue 0)
            (for _ (range 1 (+ _returnvalue 1))
              (if (`KismetMathLibrary.RandomBoolWithWeight` (`.SpawnOnStartChance_25_ADBFFAA54136194292821F816BF96193` (break `/Game/WorkbenchModsSystem/Blueprints/AI/Spawner/F_WMS_EnemySettings` _element)))
                (`self.AnyPointsLeftForThisEnemy` (`self.CachedStartPoints`) _element
                  (:`true`
                    (`self.AnyPointsLeft` _cachedstartpoints "Start Points"
                      (:`True`
                        (bind _spawnpoint (`self.SpawnEnemy` _element (`KismetArrayLibrary.Array_Random` (`self.GetRandomPoints` _cachedstartpoints)) (`KismetArrayLibrary.Array_Random` (`self.GetSpecificPoints` (`self.CachedStartPoints`) _element))))
                        (`KismetArrayLibrary.Array_RemoveItem` (`self.CachedStartPoints`) _spawnpoint))
                      (:`False`
                        (goto _label :!via `Break`)))))))))
        (:`Completed`
          (`KismetArrayLibrary.Array_Clear` (`self.CachedStartPoints`))
          (`self.SpawnRestOfEnemies`))))
    (:`then_1`
      (`self.ResetWaveGoal`))))

(event `OnUnitDead`
  (params (Unit :type "HSCharBase Object Reference") (DamageCauser :type "Actor Object Reference") (PreviousState :type "EUnitState Enum" :default "CS_Idle"))
  (bind ((`EnemiesToKill_26_E6E5E65F4034D2E1F9D801885316E757` _enemiestokill)) (break `/Game/WorkbenchModsSystem/Blueprints/AI/Spawner/F_WMS_EnemySpawnerSettings` (`self.CachedEnemySpawnerSettings`)))
  ;[1 1 1] OnUnitEvents
  (remove `HSCharBase.OnPreDead` Unit (`|CreateDelegate` :!event `OnUnitDead`))
  (`/Engine/EditorBlueprintResources/StandardMacros.DecrementInt` (`self.EnemiesAlive`)
    (:`  `
      (`/Engine/EditorBlueprintResources/StandardMacros.DecrementInt` _enemiestokill
        (:`  `
          (if (> _enemiestokill 0)
            (if (`self.bUnitInQueue`)
              (set `self.bUnitInQueue` false)
              (`self.SpawnEnemyAfterStart`))
            (else
              (`/Engine/EditorBlueprintResources/StandardMacros.DoOnce` false :!label _label_2
                (:`Completed`
                  (`KismetSystemLibrary.PrintString` "All Required Enemies Are Killed!" true true (struct :`R` 0.057249 :`G` 1.0 :`A` 1.0))
                  (`self.OnAllRequiredEnemiesAreKilled` (`.BreakTimeAfterEnd_23_8F55C3914FC45994E826048FA316C6AE` (break `/Game/WorkbenchModsSystem/Blueprints/AI/Spawner/F_WMS_EnemySpawnerSettings` (`self.CachedEnemySpawnerSettings`))))
                  (remove `/Game/WorkbenchModsSystem/Blueprints/AI/UnitFactory/BP_WMS_UnitFactory.OnUnitSpawned` (`self.UnitFactory`) (`|CreateDelegate` :!event `OnUnitSpawned`))
                  (set `self.bEnabled` false))))))))))

(event `ResetWaveGoal`
  ;[1 1 1] OnUnitEvents
  (goto _label_2 :!via `Reset`))

(event `SpawnRestOfEnemies`
  (bind ((`SpawningDynamic_30_A4B2B026460627F8883791A8BC132945` _spawningdynamic) (`SpawningDynamicCoefficent_39_3B8B9BE04AE1DD07F8FC5DBD9E853105` _spawningdynamiccoefficent)) (break `/Game/WorkbenchModsSystem/Blueprints/AI/Spawner/F_WMS_EnemySpawnerSettings` (`self.CachedEnemySpawnerSettings`)))
  ;[1 1 1] SpawnAfterStart
  (`KismetSystemLibrary.Delay` (/ (`CurveFloat.GetFloatValue` _spawningdynamic (* (- 1.0 (/ (`KismetMathLibrary.Conv_IntToDouble` (`.EnemiesToKill_26_E6E5E65F4034D2E1F9D801885316E757` (break `/Game/WorkbenchModsSystem/Blueprints/AI/Spawner/F_WMS_EnemySpawnerSettings` (`self.CachedEnemySpawnerSettings`)))) (`KismetMathLibrary.Conv_IntToDouble` (`self.EnemiesToKillRequired`)))) 100.0)) _spawningdynamiccoefficent))
  (if (`self.bEnabled`)
    (if (not (>= (`self.EnemiesAlive`) (`.MaxUnitsAlivedOnWave_42_0EDC0E15405FC3AABC5A8DA0A3753E12` (break `/Game/WorkbenchModsSystem/Blueprints/AI/Spawner/F_WMS_EnemySpawnerSettings` (`self.CachedEnemySpawnerSettings`)))))
      (`self.SpawnEnemyAfterStart`)
      (else
        (set `self.bUnitInQueue` true)))))

(event `SpawnEnemyAfterStart`
  (bind ((`EnemiesToSpawn_43_72F9EC6D4366F1317AC1069CF36B1151` _enemiestospawn)) (break `/Game/WorkbenchModsSystem/Blueprints/AI/Spawner/F_WMS_EnemySpawnerSettings` (`self.CachedEnemySpawnerSettings`)))
  ;[1 1 1] SpawnAfterStart
  (set `self.RandomEnemy` (`self.GetRandomEnemy` _enemiestospawn))
  (if (`self.IsThereAnyEnemies` _enemiestospawn)
    (`self.SpawnEnemy` (`self.RandomEnemy`) (`KismetArrayLibrary.Array_Random` (`self.GetRandomPoints` (`self.CachedAllPoints`))) (`KismetArrayLibrary.Array_Random` (`self.GetSpecificPoints` (`self.CachedAllPoints`) (`self.RandomEnemy`))))
    (`self.SpawnRestOfEnemies`)
    (else
      (`KismetSystemLibrary.PrintString` "All Enemies Are Spawned!" true true (struct :`G` 0.333552 :`B` 1.0 :`A` 1.0)))))

(fn `DecrementSpawnAmount`
  (params (PresetName :type Name))
  (bind ((`EnemiesToSpawn_43_72F9EC6D4366F1317AC1069CF36B1151` _enemiestospawn)) (break `/Game/WorkbenchModsSystem/Blueprints/AI/Spawner/F_WMS_EnemySpawnerSettings` (`self.CachedEnemySpawnerSettings`)))
  (`/Engine/EditorBlueprintResources/StandardMacros.DecrementInt` (`.MaxToSpawn_19_63846AB7475BF2D8B145BCA912440D96` (break `/Game/WorkbenchModsSystem/Blueprints/AI/Spawner/F_WMS_EnemySettings` (`|GetArrayItem` _enemiestospawn (`KismetArrayLibrary.Array_Find` _enemiestospawn (`self.GetEnemyByPresetName` (`local.PresetName`) (`.EnemiesToSpawn_43_72F9EC6D4366F1317AC1069CF36B1151` (break `/Game/WorkbenchModsSystem/Blueprints/AI/Spawner/F_WMS_EnemySpawnerSettings` (`self.CachedEnemySpawnerSettings`))))))))))

(fn `FillSpawnerDataFromTable`
  (`/Engine/EditorBlueprintResources/StandardMacros.IsValid` (`self.SpawnerPresetsTable`)
    (:`Is Valid`
      (`BlueprintMapLibrary.Map_Clear` (`self.EnemiesById`))
      (bind _outrownames (`DataTableFunctionLibrary.GetDataTableRowNames` (`self.SpawnerPresetsTable`)))
      (for (_array_element _array_index) _outrownames
        (bind _returnvalue (`|GetDataTableRow` (`self.SpawnerPresetsTable`) _array_element)
          (:`then`
            (`BlueprintMapLibrary.Map_Add` (`self.EnemiesById`) (+ _array_index 1) _returnvalue))))
      (return))))

(fn `ForceEnemiesSpawn`
  (params (Id :type Integer))
  (returns (Success :type Boolean))
  (if (not (`self.bEnabled`))
    (set `self.bEnabled` true)
    (`self.InitializeSpawnPoints`)
    (`self.AnyPointsLeft` (`self.CachedAllPoints`) "All Points"
      (:`True`
        (bind _success (`self.SpawnEnemiesById` (`local.Id`)))
        (return _success)))
    (else
      (`KismetSystemLibrary.PrintString` "Spawner already working!" true true (struct :`R` 1.0 :`B` 0.007519 :`A` 1.0))
      (return true))))

(fn `GetEnemyByPresetName`
  (params (PresetName :type Name) (EnemiesArray :type "Array of /Game/WorkbenchModsSystem/Blueprints/AI/Spawner/F_WMS_EnemySettings Structure"))
  (returns (Enemy :type "/Game/WorkbenchModsSystem/Blueprints/AI/Spawner/F_WMS_EnemySettings Structure"))
  (for _array_element (`local.EnemiesArray`)
    (if (== (`.EnemyPresetName_10_3303B1914B18FD6742E55E992EDF6ED3` (break `/Game/WorkbenchModsSystem/Blueprints/AI/Spawner/F_WMS_EnemySettings` _array_element)) (`local.PresetName`))
      (return _array_element)))
  (`KismetSystemLibrary.PrintString` "EnemyPreset Not Found" true true (struct :`R` 1.0 :`G` 0.396118 :`A` 1.0))
  (return))

(fn `GetRandomEnemy`
  (params (Enemies :type "Array of /Game/WorkbenchModsSystem/Blueprints/AI/Spawner/F_WMS_EnemySettings Structure"))
  (returns (RandomEnemy :type "/Game/WorkbenchModsSystem/Blueprints/AI/Spawner/F_WMS_EnemySettings Structure"))
  (locals (EnemiesByRatio :type "Array of Float (double-precision)") (TotalRatio :type "Float (double-precision)" :default 0.0) (RatioRange :type "Array of Float (double-precision)") (EnemiesThatCanBeSpawned :type "Array of /Game/WorkbenchModsSystem/Blueprints/AI/Spawner/F_WMS_EnemySettings Structure") (Enemy :type "/Game/WorkbenchModsSystem/Blueprints/AI/Spawner/F_WMS_EnemySettings Structure"))
  (for _array_element Enemies
    (bind ((`MaxToSpawn_19_63846AB7475BF2D8B145BCA912440D96` _maxtospawn) (`SpawnRatio_22_B0831F3D4930E3BDD893E8A62A1C8897` _spawnratio)) (break `/Game/WorkbenchModsSystem/Blueprints/AI/Spawner/F_WMS_EnemySettings` _array_element))
    (if (> _maxtospawn 0)
      (`KismetArrayLibrary.Array_Add` (`local.EnemiesByRatio`) _spawnratio)
      (`KismetArrayLibrary.Array_Add` (`local.EnemiesThatCanBeSpawned`) _array_element)))
  (for _array_element_2 (`local.EnemiesByRatio`)
    (bind _output_get (set `local.TotalRatio` (+ _array_element_2 (`local.TotalRatio`))))
    (`KismetArrayLibrary.Array_Add` (`local.RatioRange`) _output_get))
  (for (_array_element_3 _array_index) (`local.RatioRange`)
    (if (> _array_element_3 (`KismetMathLibrary.RandomFloatInRange` 0.0 (`local.TotalRatio`)))
      (bind _output_get_2 (set `local.Enemy` (`|GetArrayItem` (`local.EnemiesThatCanBeSpawned`) _array_index)))
      (return _output_get_2)))
  (`KismetSystemLibrary.PrintString` "Enemies Not Found" true true (struct :`R` 1.0 :`G` 0.1648 :`A` 1.0) 5.0)
  (return))

(fn `GetRandomPoints`
  (params (Points :type "Array of /Game/WorkbenchModsSystem/Blueprints/AI/Spawner/BP_WMS_EnemySpawnPoint Object Reference"))
  (returns (RandomPoints :type "Array of /Game/WorkbenchModsSystem/Blueprints/AI/Spawner/BP_WMS_EnemySpawnPoint Object Reference"))
  (locals (CachedRandomPoints :type "Array of /Game/WorkbenchModsSystem/Blueprints/AI/Spawner/BP_WMS_EnemySpawnPoint Object Reference"))
  (for _array_element Points
    (if (`/Game/WorkbenchModsSystem/Blueprints/AI/Spawner/BP_WMS_EnemySpawnPoint.bRandomPoint` _array_element)
      (`KismetArrayLibrary.Array_Add` (`local.CachedRandomPoints`) _array_element)))
  (return (`local.CachedRandomPoints`)))

(fn `GetSpecificPoints`
  (params (Points :type "Array of /Game/WorkbenchModsSystem/Blueprints/AI/Spawner/BP_WMS_EnemySpawnPoint Object Reference") (EnemyPreset :type "/Game/WorkbenchModsSystem/Blueprints/AI/Spawner/F_WMS_EnemySettings Structure"))
  (returns (SpecificPoints :type "Array of /Game/WorkbenchModsSystem/Blueprints/AI/Spawner/BP_WMS_EnemySpawnPoint Object Reference"))
  (locals (CachedSpecificPoints :type "Array of /Game/WorkbenchModsSystem/Blueprints/AI/Spawner/BP_WMS_EnemySpawnPoint Object Reference"))
  (for _array_element Points
    (for _array_element_2 (`/Game/WorkbenchModsSystem/Blueprints/AI/Spawner/BP_WMS_EnemySpawnPoint.SpecificPresets` _array_element)
      (if (== (`.RowName` (break `DataTableRowHandle` _array_element_2)) (`.EnemyPresetName_10_3303B1914B18FD6742E55E992EDF6ED3` (break `/Game/WorkbenchModsSystem/Blueprints/AI/Spawner/F_WMS_EnemySettings` (`local.EnemyPreset`))))
        (`KismetArrayLibrary.Array_Add` (`local.CachedSpecificPoints`) _array_element))))
  (return (`local.CachedSpecificPoints`)))

(fn `InitializeSpawnPoints`
  (if (not (`self.bInitialized`))
    (bind _outactors (`GameplayStatics.GetAllActorsOfClass` "/Game/WorkbenchModsSystem/Blueprints/AI/Spawner/BP_WMS_EnemySpawnPoint.BP_WMS_EnemySpawnPoint_C"))
    (for _array_element _outactors
      (if (or (> (`KismetArrayLibrary.Array_Length` (`/Game/WorkbenchModsSystem/Blueprints/AI/Spawner/BP_WMS_EnemySpawnPoint.SpecificPresets` _array_element)) 0) (`/Game/WorkbenchModsSystem/Blueprints/AI/Spawner/BP_WMS_EnemySpawnPoint.bRandomPoint` _array_element))
        (`KismetArrayLibrary.Array_Add` (`self.CachedAllPoints`) _array_element)))
    (set `self.bInitialized` true)
    (`self.OnSpawnPointsInitialized`)
    (return)
    (else
      (return))))

(fn `IsThereAnyEnemies`
  (params (Enemies :type "Array of /Game/WorkbenchModsSystem/Blueprints/AI/Spawner/F_WMS_EnemySettings Structure"))
  (returns (Condition :type Boolean))
  (for _array_element Enemies
    (if (> (`.MaxToSpawn_19_63846AB7475BF2D8B145BCA912440D96` (break `/Game/WorkbenchModsSystem/Blueprints/AI/Spawner/F_WMS_EnemySettings` _array_element)) 0)
      (return true)))
  (return false))

(fn `SortEnemies`
  (params (EnemiesToSpawn :type "Array of /Game/WorkbenchModsSystem/Blueprints/AI/Spawner/F_WMS_EnemySettings Structure (by ref)"))
  (returns (EnemiesToSpawnResorted :type "Array of /Game/WorkbenchModsSystem/Blueprints/AI/Spawner/F_WMS_EnemySettings Structure (by ref)"))
  (locals (SortedArray :type "Array of /Game/WorkbenchModsSystem/Blueprints/AI/Spawner/F_WMS_EnemySettings Structure"))
  (for _array_element EnemiesToSpawn
    (if (!= (`KismetArrayLibrary.Array_Length` (`self.GetSpecificPoints` (`self.CachedAllPoints`) _array_element)) 0)
      (`KismetArrayLibrary.Array_Insert` (`local.SortedArray`) _array_element)
      (else
        (`KismetArrayLibrary.Array_Add` (`local.SortedArray`) _array_element))))
  (return (`local.SortedArray`)))

(fn `SpawnEnemiesById`
  (params (Id :type Integer))
  (returns (Success :type Boolean))
  (bind (_enemiestospawn _enemiestokill) (break `/Game/WorkbenchModsSystem/Blueprints/AI/Spawner/F_WMS_EnemySpawnerSettings` (`self.CachedEnemySpawnerSettings`)))
  (bind _enemyspawner (`self.HasEnemiesForThisId` Id)
    (:`true`
      (set `self.CachedEnemySpawnerSettings` _enemyspawner)
      (set `self.EnemiesToKillRequired` _enemiestokill)
      (add `/Game/WorkbenchModsSystem/Blueprints/AI/UnitFactory/BP_WMS_UnitFactory.OnUnitSpawned` (`self.UnitFactory`) (`|CreateDelegate` :!event `OnUnitSpawned`))
      (bind _enemiestospawnresorted (`self.SortEnemies` _enemiestospawn))
      (`|VariableSetRef` (`.EnemiesToSpawn_43_72F9EC6D4366F1317AC1069CF36B1151` (break `/Game/WorkbenchModsSystem/Blueprints/AI/Spawner/F_WMS_EnemySpawnerSettings` (`self.CachedEnemySpawnerSettings`))) _enemiestospawnresorted)
      (`self.SpawnAtTheStart`)
      (return true))
    (:`false`
      (return false))))

(fn `SpawnEnemy`
  (params (EnemyToSpawn :type "/Game/WorkbenchModsSystem/Blueprints/AI/Spawner/F_WMS_EnemySettings Structure") (RandomPoint :type "/Game/WorkbenchModsSystem/Blueprints/AI/Spawner/BP_WMS_EnemySpawnPoint Object Reference") (SpecificPoint :type "/Game/WorkbenchModsSystem/Blueprints/AI/Spawner/BP_WMS_EnemySpawnPoint Object Reference"))
  (returns (SpawnPoint :type "/Game/WorkbenchModsSystem/Blueprints/AI/Spawner/BP_WMS_EnemySpawnPoint Object Reference"))
  (locals (ChoosenPoint :type "/Game/WorkbenchModsSystem/Blueprints/AI/Spawner/BP_WMS_EnemySpawnPoint Object Reference"))
  (set `local.ChoosenPoint` (select `bool` (`KismetSystemLibrary.IsValid` (`local.SpecificPoint`)) :`false` (`local.RandomPoint`) :`true` (`local.SpecificPoint`)))
  (`/Game/WorkbenchModsSystem/Blueprints/AI/UnitFactory/BP_WMS_UnitFactory.SpawnUnitFromPreset` (`self.UnitFactory`) (`.EnemyPresetName_10_3303B1914B18FD6742E55E992EDF6ED3` (break `/Game/WorkbenchModsSystem/Blueprints/AI/Spawner/F_WMS_EnemySettings` (`local.EnemyToSpawn`))) (`KismetMathLibrary.MakeTransform` (`self.K2_GetActorLocation` (`local.ChoosenPoint`))))
  (return (`local.ChoosenPoint`)))

(fn `UserConstructionScript`)