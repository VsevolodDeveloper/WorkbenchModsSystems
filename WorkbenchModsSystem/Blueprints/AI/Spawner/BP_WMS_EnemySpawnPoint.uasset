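; BP_WMS_EnemySpawnPoint is an enemy spawn point that keeps its list of specific unit presets pointed at the spawner's preset table.
; SetNewPresets finds a BP_WMS_EnemySpawner in the level, validates its unit factory and UnitPresetsData, then rewrites each SpecificPresets handle to that DataTable while keeping the row name.
; This sync runs in the Construction Script and again shortly after BeginPlay, following a brief delay.
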(event `self.ReceiveBeginPlay`
  (`KismetSystemLibrary.Delay` 0.2)
  (`self.SetNewPresets`))

(fn `SetNewPresets`
  (bind _returnvalue (`GameplayStatics.GetActorOfClass` "/Game/WorkbenchModsSystem/Blueprints/AI/Spawner/BP_WMS_EnemySpawner.BP_WMS_EnemySpawner_C"))
  (`/Engine/EditorBlueprintResources/StandardMacros.IsValid` _returnvalue
    (:`Is Valid`
      (bind _unitfactory (`/Game/WorkbenchModsSystem/Blueprints/AI/Spawner/BP_WMS_EnemySpawner.UnitFactory` _returnvalue))
      (if (and (`KismetSystemLibrary.IsValidClass` (`/Game/WorkbenchModsSystem/Blueprints/AI/Spawner/BP_WMS_EnemySpawner.UnitFactoryClass` _returnvalue)) (`KismetSystemLibrary.IsValid` _unitfactory))
        (bind _unitpresetsdata (`/Game/WorkbenchModsSystem/Blueprints/AI/UnitFactory/BP_WMS_UnitFactory.UnitPresetsData` _unitfactory))
        (`/Engine/EditorBlueprintResources/StandardMacros.IsValid` _unitpresetsdata
          (:`Is Valid`
            (for (_array_element _array_index) (`self.SpecificPresets`)
              (`KismetArrayLibrary.Array_Set` (`self.SpecificPresets`) _array_index (make `DataTableRowHandle` _unitpresetsdata (`.RowName` (break `DataTableRowHandle` _array_element)))))))))))

(fn `UserConstructionScript`
  (`self.SetNewPresets`))