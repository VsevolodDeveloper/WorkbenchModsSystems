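; Points manager that overrides the spawn points used by the WMS enemy spawner with a set selected by ID.
; SetSpawnPoints looks up an ID in PointsByID and stores that entry's points as the pending array.
; On BeginPlay it finds the spawner and binds to its points-initialized event.
; When that event fires, a non-empty pending array replaces the spawner's cached points and clears its Initialized flag.
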(event `self.ReceiveBeginPlay`
  (bind _returnvalue (`GameplayStatics.GetActorOfClass` "/Game/WorkbenchModsSystem/Blueprints/AI/Spawner/BP_WMS_EnemySpawner.BP_WMS_EnemySpawner_C"))
  (bind _output_get (set `self.EnemySpawner` _returnvalue))
  (add `/Game/WorkbenchModsSystem/Blueprints/AI/Spawner/BP_WMS_EnemySpawner.OnSpawnPointsInitialized` _output_get (delegate `OnSpawnPointsInitialized`)))

(event `OnSpawnPointsInitialized`
  (if (`KismetArrayLibrary.Array_IsValidIndex` (`self.PointsToSet`))
    (set `/Game/WorkbenchModsSystem/Blueprints/AI/Spawner/BP_WMS_EnemySpawner.CachedAllPoints` (`self.PointsToSet`) (`self.EnemySpawner`))
    (set `/Game/WorkbenchModsSystem/Blueprints/AI/Spawner/BP_WMS_EnemySpawner.bInitialized` false (`self.EnemySpawner`))))

(event `SetSpawnPoints`
  (params (ID :type Integer))
  (bind _result (`BlueprintSetLibrary.Set_ToArray` (`.Points_3_687D156B48E86BB0AF4DFE9C6D1CF809` (break `/Game/WorkbenchModsSystem/Blueprints/AI/Spawner/PointsManager/F_WMS_ControlledPoints` (`|GetArrayItem` (`self.PointsByID`) ID)))))
  (set `self.PointsToSet` _result))

(fn `UserConstructionScript`)