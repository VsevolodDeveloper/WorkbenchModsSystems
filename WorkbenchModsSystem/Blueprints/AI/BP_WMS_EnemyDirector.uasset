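; Enemy director that tracks living units and the target's current volume, which serves as the molotov-throw check.
; It gathers existing HSCharBase actors at start, adds units spawned by BP_WMS_UnitFactory, and removes those spawned units on pre-death.
; It rebroadcasts deaths and volume enter/leave changes as events.
; SetBoolKeyForEnemy writes a blackboard bool to a given enemy, or picks a random one by class or from living units.
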(event `self.ReceiveBeginPlay`
  (`KismetSystemLibrary.Delay` 0.2)
  (bind _returnvalue (`GameplayStatics.GetActorOfClass` "/Game/WorkbenchModsSystem/Blueprints/AI/UnitFactory/BP_WMS_UnitFactory.BP_WMS_UnitFactory_C"))
  (`/Engine/EditorBlueprintResources/StandardMacros.IsValid` _returnvalue
    (:`Is Valid`
      (add `/Game/WorkbenchModsSystem/Blueprints/AI/UnitFactory/BP_WMS_UnitFactory.OnUnitSpawned` _returnvalue (delegate `OnUnitSpawned`)))
    (:`Is Not Valid`
      _))
  (bind _outactors (`GameplayStatics.GetAllActorsOfClass` "/Script/Hellsplit_Arena.HSCharBase"))
  (`KismetArrayLibrary.Array_Append` (`self.AlivedUnits`) _outactors))

(event `OnUnitSpawned`
  (params (Unit :type "Actor Object Reference") (UnitPresetName :type Name) (Success :type Boolean))
  (if Success
    (bind _ashschar_base (cast `HSCharBase` Unit))
    (`KismetArrayLibrary.Array_AddUnique` (`self.AlivedUnits`) _ashschar_base)
    (add `HSCharBase.OnPreDead` _ashschar_base (delegate `OnUnitDead`))))

(event `OnUnitDead`
  (params (Unit :type "HSCharBase Object Reference") (DamageCauser :type "Actor Object Reference") (PreviousState :type "EUnitState Enum" :default "CS_Idle"))
  (`KismetArrayLibrary.Array_RemoveItem` (`self.AlivedUnits`) Unit)
  (`self.OnAnyUnitDead` Unit DamageCauser PreviousState))

(event `UpdateCurrentTargetVolume`
  (params (Volume :type "Actor Object Reference") (bEntered :type Boolean))
  (bind _volumewheretargetislocated (`self.VolumeWhereTargetIsLocated`))
  (bind _output_get (set `self.VolumeWhereTargetIsLocated` Volume))
  (`/Engine/EditorBlueprintResources/StandardMacros.IsValid` _output_get
    (:`Is Valid`
      (if bEntered
        (`self.OnTargetEnteredNewVolume` _volumewheretargetislocated)
        (else
          (`self.OnTargetLeaveVolume` _volumewheretargetislocated))))))

(fn `GetCurrentTargetVolume`
  (returns (VolumeWhereTargetIsLocated :type "Actor Object Reference"))
  (return (`self.VolumeWhereTargetIsLocated`)))

(fn `IsPlayerInThrowMolotovVolume`
  (returns (ReturnValue :type Boolean))
  (return (`KismetSystemLibrary.IsValid` (`self.VolumeWhereTargetIsLocated`))))

(fn `SetBoolKeyForEnemy`
  (params (KeyName :type "Name (by ref)") (BoolValue :type Boolean) (EnemyClass :type "Actor Class Reference") (Enemy :type "Actor Object Reference"))
  (returns (ChosenEnemy :type "Actor Object Reference"))
  (locals (RandomEnemy :type "Actor Object Reference"))
  (bind _returnvalue (`AIBlueprintHelperLibrary.GetBlackboard` (`AIBlueprintHelperLibrary.GetAIController` (`local.RandomEnemy`))))
  (bind _returnvalue_2 (`AIBlueprintHelperLibrary.GetBlackboard` (`AIBlueprintHelperLibrary.GetAIController` (`KismetArrayLibrary.Array_Random` (`self.AlivedUnits`)))))
  (`/Engine/EditorBlueprintResources/StandardMacros.IsValid` Enemy
    (:`Is Valid`
      (`BlackboardComponent.SetValueAsBool` (`AIBlueprintHelperLibrary.GetBlackboard` (`AIBlueprintHelperLibrary.GetAIController` (`local.Enemy`))) (`local.KeyName`) (`local.BoolValue`))
      (return (`local.Enemy`)))
    (:`Is Not Valid`
      (if (`KismetSystemLibrary.IsValidClass` (`local.EnemyClass`))
        (bind _outactors (`GameplayStatics.GetAllActorsOfClass` (`local.EnemyClass`)))
        (bind _output_get (set `local.RandomEnemy` (`KismetArrayLibrary.Array_Random` _outactors)))
        (if (`KismetArrayLibrary.Array_Contains` (`self.AlivedUnits`) _output_get)
          (`/Engine/EditorBlueprintResources/StandardMacros.IsValid` _returnvalue
            (:`Is Valid`
              (`BlackboardComponent.SetValueAsBool` _returnvalue (`local.KeyName`) (`local.BoolValue`))
              (return (`local.RandomEnemy`))))
          (else
            _)))
      (`/Engine/EditorBlueprintResources/StandardMacros.IsValid` _returnvalue_2
        (:`Is Valid`
          (`BlackboardComponent.SetValueAsBool` _returnvalue_2 (`local.KeyName`) (`local.BoolValue`))
          (return (`local.RandomEnemy`)))))))

(fn `UserConstructionScript`)