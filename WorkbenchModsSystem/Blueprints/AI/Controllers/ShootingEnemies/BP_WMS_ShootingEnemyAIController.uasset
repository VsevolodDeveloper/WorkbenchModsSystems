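; AI controller for shooting enemies that decides which seen pawns become targets, with support for controlling teammate units.
; Non-teammates target the player directly; other sightings pass alive checks, plus an opposite-side check for WMS ALS characters.
; Accepted targets update the blackboard, notify via an any-unit-saw-target call and have death events bound to clear target and aiming.
; Being hit by anyone but the current target makes the controller instantly see the attacker.
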(event `OnSeeTarget`
  (params (Pawn :type "Pawn Object Reference"))
  (set `self.SuspiciosPawn` Pawn)
  (if (`self.bControlledPawnIsTeammate`)
    (`self.CheckThePawnIdentity`)
    (else
      (bind _ashsplayer_avatar (cast `HSPlayerAvatar` (`self.SuspiciosPawn`))
        (:`then`
          (add `HSVRCharacter.OnDead` _ashsplayer_avatar (`|CreateDelegate` :!event `OnPlayerDead`))
          (`self.SetTargetDependencies` (`self.SuspiciosPawn`)))
        (:`CastFailed`
          (`self.CheckThePawnIdentity`))))))

(event `CheckThePawnIdentity`
  (bind _asbp_wms_simple_als_base_character (cast `/Game/WorkbenchModsSystem/Blueprints/Units/BaseUnits/BP_WMS_Simple_ALS_Base_Character` (`self.SuspiciosPawn`))
    (:`then`
      (`self.CheckIsUnitAlive` _asbp_wms_simple_als_base_character
        (:`True`
          (if (!= (`/Game/WorkbenchModsSystem/Blueprints/Units/BaseUnits/BP_WMS_Simple_ALS_Base_Character.bTeammate` _asbp_wms_simple_als_base_character) (`self.bControlledPawnIsTeammate`))
            (add `HSCharBase.OnPreDead` _asbp_wms_simple_als_base_character (`|CreateDelegate` :!event `OnTargetDead`))
            (`self.SetTargetDependencies` (`self.SuspiciosPawn`) :!label _label)))))
    (:`CastFailed`
      (bind _asals_base_character (cast `/Game/Blueprints/Units/ALS_BaseCharacter` (`self.SuspiciosPawn`)))
      (`self.CheckIsUnitAlive` _asals_base_character
        (:`True`
          (add `HSCharBase.OnPreDead` _asals_base_character (`|CreateDelegate` :!event `OnTargetDead`))
          (goto _label))))))

(event `OnEnemyHit`
  (params (HitCauser :type "Actor Object Reference"))
  (if (!= HitCauser (`self.GetTarget_BB`))
    (`self.InstantlySeeTarget` HitCauser)))

(event `OnPlayerDead`
  (`self.SetTarget` null)
  (`self.SetKnowAboutTarget_BB` false)
  (`self.SetAiming_BB` false))

(event `OnTargetDead`
  (params (Unit :type "HSCharBase Object Reference") (DamageCauser :type "Actor Object Reference") (PreviousState :type "EUnitState Enum" :default "CS_Idle"))
  (`KismetSystemLibrary.Delay` 3.0)
  (`self.SetTarget` null)
  (`self.SetKnowAboutTarget_BB` false)
  (`self.SetAiming_BB` false))

(fn `GetAiming_BB`
  (returns (ReturnValue :type Boolean))
  (bind _returnvalue (`AIBlueprintHelperLibrary.GetBlackboard` null))
  (`/Engine/EditorBlueprintResources/StandardMacros.IsValid` _returnvalue
    (:`Is Valid`
      (return (`BlackboardComponent.GetValueAsBool` _returnvalue "Aiming")))))

(fn `Initialize`
  (`parent.Initialize`)
  (bind _asbp_wms_simple_als_base_character (cast `/Game/WorkbenchModsSystem/Blueprints/Units/BaseUnits/BP_WMS_Simple_ALS_Base_Character` (`self.PossessedPawn`)))
  (add `/Game/WorkbenchModsSystem/Blueprints/Units/BaseUnits/BP_WMS_Simple_ALS_Base_Character.OnEnemyHit` _asbp_wms_simple_als_base_character (`|CreateDelegate` :!event `OnEnemyHit`)))

(fn `SetAiming_BB`
  (params (Aiming :type Boolean))
  (`BlackboardComponent.SetValueAsBool` (`AIBlueprintHelperLibrary.GetBlackboard` null) "Aiming" (`local.Aiming`)))

(fn `SetTargetDependencies`
  (params (InTarget :type "Pawn Object Reference"))
  (`parent.OnSeeTarget` InTarget)
  (`self.SetKnowAboutTarget_BB` true)
  (`self.SetTarget` (`local.InTarget`))
  (`self.CallOnAnyUnitSawTarget`))

(fn `UserConstructionScript`)