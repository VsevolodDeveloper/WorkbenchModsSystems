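; AI controller for medieval team units in the Workbench mods system that instantly kills its unit once it loses a limb segment.
; It caches the possessed ALS character when the blackboard starts, then checks its injury component every tick.
; A missing thigh or shin also clears the CanWalk blackboard key.
; Any missing leg, forearm or shoulder part triggers Kill on the character.
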(event `self.ReceiveTick`
  (params (DeltaSeconds :type "Float (single-precision)"))
  (`parent.ReceiveTick` DeltaSeconds)
  (`self.PerformInstantDeath`))

(event `self.OnUsingBlackBoard`
  (params (BlackboardComp :type "BlackboardComponent Object Reference") (BlackboardAsset :type "BlackboardData Object Reference"))
  (`parent.OnUsingBlackBoard` BlackboardComp BlackboardAsset)
  (bind _asals_base_character (cast `/Game/Blueprints/Units/ALS_BaseCharacter` (`self.PossessedPawn`)))
  (set `self.PossedPawnAsALS_BaseCharacter` _asals_base_character))

(fn `CheckCanWalk`
  (returns (bResult :type Boolean))
  (bind _returnvalue (`AIBlueprintHelperLibrary.GetBlackboard` null))
  (`self.PossedPawnAsALS_BaseCharacter`
    (:`then`
      (if (or (not (`HSUnitInjuriesComponent.IsBodyPartExists` (`HSCharBase.UnitInjuries` (`self.PossedPawnAsALS_BaseCharacter`)) "femur_r" false)) (not (`HSUnitInjuriesComponent.IsBodyPartExists` (`HSCharBase.UnitInjuries` (`self.PossedPawnAsALS_BaseCharacter`)) "femur_l" false)) (not (`HSUnitInjuriesComponent.IsBodyPartExists` (`HSCharBase.UnitInjuries` (`self.PossedPawnAsALS_BaseCharacter`)) "shin_l" false)) (not (`HSUnitInjuriesComponent.IsBodyPartExists` (`HSCharBase.UnitInjuries` (`self.PossedPawnAsALS_BaseCharacter`)) "shin_r" false)))
        (`/Engine/EditorBlueprintResources/StandardMacros.IsValid` _returnvalue
          (:`Is Valid`
            (`BlackboardComponent.SetValueAsBool` _returnvalue "CanWalk" false)
            (return false)))
        (else
          (return true))))
    (:`else`)))

(fn `CheckHasHands`
  (returns (bResult :type Boolean))
  (`self.PossedPawnAsALS_BaseCharacter`
    (:`then`
      (if (or (not (`HSUnitInjuriesComponent.IsBodyPartExists` (`HSCharBase.UnitInjuries` (`self.PossedPawnAsALS_BaseCharacter`)) "forearm_r" false)) (not (`HSUnitInjuriesComponent.IsBodyPartExists` (`HSCharBase.UnitInjuries` (`self.PossedPawnAsALS_BaseCharacter`)) "forearm_l" false)) (not (`HSUnitInjuriesComponent.IsBodyPartExists` (`HSCharBase.UnitInjuries` (`self.PossedPawnAsALS_BaseCharacter`)) "shoulder_r" false)) (not (`HSUnitInjuriesComponent.IsBodyPartExists` (`HSCharBase.UnitInjuries` (`self.PossedPawnAsALS_BaseCharacter`)) "shoulder_l" false)))
        (return false)
        (else
          (return true))))
    (:`else`)))

(fn `PerformInstantDeath`
  (bind _bresult (`self.CheckCanWalk`))
  (if (not (and _bresult (`self.CheckHasHands`)))
    (bind _possedpawnasals_basecharacter (`self.PossedPawnAsALS_BaseCharacter`)
      (:`then`
        (`HSCharBase.Kill` _possedpawnasals_basecharacter ""))
      (:`else`))))

(fn `UserConstructionScript`
  (`parent.UserConstructionScript`))