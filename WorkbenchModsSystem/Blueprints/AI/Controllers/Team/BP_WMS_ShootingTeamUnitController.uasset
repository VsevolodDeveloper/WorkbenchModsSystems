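; AI controller for team-based shooting units that manages the blackboard target and aiming state.
; It caches all pawns, updating the list on spawn and death events, and uses it to alert opposing AI within range when its pawn shoots.
; Being hit makes it instantly target the attacker.
; Target or player death clears targeting after a short delay, and target death also triggers a check for teammates needing help.
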(event `OnEnemyHit`
  (params (HitCauser :type "Actor Object Reference"))
  (if (!= HitCauser (`self.GetTarget_BB`))
    (`self.InstantlySeeTarget` HitCauser)))

(event `self.OnPlayerDead`
  (`KismetArrayLibrary.Array_RemoveItem` (`self.CachedUnits`) (`GameplayStatics.GetPlayerPawn` 0))
  (`KismetSystemLibrary.Delay` 2.0)
  (`self.SetTarget_BB` null)
  (`self.SetTarget` null)
  (`self.SetKnowAboutTarget_BB` false)
  (`self.SetAiming_BB` false))

(event `self.OnTargetDead`
  (params (Unit :type "HSCharBase Object Reference") (DamageCauser :type "Actor Object Reference") (PreviousState :type "EUnitState Enum" :default "CS_Idle"))
  (`KismetSystemLibrary.Delay` 0.5)
  (`self.SetTarget_BB` null)
  (`self.SetTarget` null)
  (`self.SetKnowAboutTarget_BB` false)
  (`self.SetAiming_BB` false)
  (`self.CheckIfTeammatesNeedsHelp`))

(event `InitializeCachedUnits`
  (`|ExecutionSequence`
    (:`then_0`
      (bind _outactors (`GameplayStatics.GetAllActorsOfClass` "/Script/Engine.Pawn"))
      (bind _output_get (set `self.CachedUnits` _outactors))
      (for _array_element _output_get
        (bind _ashschar_base (cast `HSCharBase` _array_element)
          (:`then`
            (add `HSCharBase.OnPostDead` _ashschar_base (`|CreateDelegate` :!event `OnCachedUnitDead`)))
          (:`CastFailed`
            (bind _ashsplayer_avatar (cast `HSPlayerAvatar` _array_element))
            (add `HSVRCharacter.OnDead` _ashsplayer_avatar (`|CreateDelegate` :!event `OnPlayerDead`))))))))

(event `OnCachedUnitDead`
  (params (Unit :type "HSCharBase Object Reference") (DamageCauser :type "Actor Object Reference") (PreviousState :type "EUnitState Enum" :default "CS_Idle"))
  (`KismetArrayLibrary.Array_RemoveItem` (`self.CachedUnits`) Unit))

(event `OnCachedUnitSpawned`
  (params (ShootingEnemyBase :type "Pawn Object Reference"))
  (`KismetArrayLibrary.Array_Add` (`self.CachedUnits`) ShootingEnemyBase)
  (bind _ashschar_base (cast `HSCharBase` ShootingEnemyBase))
  (add `HSCharBase.OnPostDead` _ashschar_base (`|CreateDelegate` :!event `OnCachedUnitDead`)))

(event `OnPlayerSpawned`
  (params (Player :type "Pawn Object Reference"))
  (`KismetArrayLibrary.Array_Add` (`self.CachedUnits`) Player)
  (bind _ashsplayer_avatar (cast `HSPlayerAvatar` Player))
  (add `HSVRCharacter.OnDead` _ashsplayer_avatar (`|CreateDelegate` :!event `OnPlayerDead`)))

(fn `GetAiming_BB`
  (returns (ReturnValue :type Boolean))
  (bind _returnvalue (`AIBlueprintHelperLibrary.GetBlackboard` null))
  (`/Engine/EditorBlueprintResources/StandardMacros.IsValid` _returnvalue
    (:`Is Valid`
      (return (`BlackboardComponent.GetValueAsBool` _returnvalue "Aiming")))))

(fn `Initialize`
  (`parent.Initialize`)
  (`self.InitializeCachedUnits`)
  (bind _asbp_wms_simple_als_base_character (cast `/Game/WorkbenchModsSystem/Blueprints/Units/BaseUnits/BP_WMS_Simple_ALS_Base_Character` (`self.PossessedPawn`)))
  (add `/Game/WorkbenchModsSystem/Blueprints/Units/BaseUnits/BP_WMS_Simple_ALS_Base_Character.OnEnemyHit` _asbp_wms_simple_als_base_character (`|CreateDelegate` :!event `OnEnemyHit`)))

(fn `NotifyAllEnmiesAboutShooting`
  (for _array_element (`self.CachedUnits`)
    (`/Engine/EditorBlueprintResources/StandardMacros.IsValid` _array_element
      (:`Is Valid`
        (if (< (`self.GetDistanceTo` (`self.PossessedPawn`) _array_element) 2500.0)
          (bind _bunitisteammate (message `/Game/WorkbenchModsSystem/Blueprints/Interfaces/BPI_WMS_UnitInterface.GetUnitIsTeammate` _array_element))
          (if (!= _bunitisteammate (`self.bControlledPawnIsTeammate`))
            (bind _asbp_wms_simple_aicontroller (cast `/Game/WorkbenchModsSystem/Blueprints/AI/Controllers/BP_WMS_SimpleAIController` (`Pawn.GetController` _array_element)))
            (if (not (`self.GetKnowAboutTarget_BB` _asbp_wms_simple_aicontroller))
              (`self.InstantlySeeTarget` _asbp_wms_simple_aicontroller (`self.PossessedPawn`)))))))))

(fn `SetAiming_BB`
  (params (Aiming :type Boolean))
  (`BlackboardComponent.SetValueAsBool` (`AIBlueprintHelperLibrary.GetBlackboard` null) "Aiming" (`local.Aiming`)))

(fn `SetTargetDependencies`
  (params (InTarget :type "Pawn Object Reference"))
  (`parent.SetTargetDependencies` InTarget)
  (`self.SetAiming_BB` true))

(fn `UserConstructionScript`)