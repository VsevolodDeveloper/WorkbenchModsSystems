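; AI controller for team-based units that picks combat targets by teammate flag, fighting either allies of the player or enemies.
; Sighted opposing units become blackboard targets; non-teammates prioritize the player, otherwise closer sightings can replace known targets through a cooldown gate.
; Death events clear targets after a delay; after unit kills, it adopts a nearby engaged teammate's target.
; Box traces support that search and random enemy selection across a wide area.
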(event `self.OnSeeTarget`
  (params (Pawn :type "Pawn Object Reference"))
  (set `self.SuspiciosPawn` Pawn)
  (if (`self.bControlledPawnIsTeammate`)
    (`self.CheckThePawnIdentity`)
    (else
      (cast `HSPlayerAvatar` (`self.GetTarget_BB`)
        (:`CastFailed`
          (bind _ashsplayer_avatar (cast `HSPlayerAvatar` (`self.SuspiciosPawn`))
            (:`then`
              (add `HSVRCharacter.OnDead` _ashsplayer_avatar (`|CreateDelegate` :!event `OnPlayerDead`))
              (`self.SetTargetDependencies` (`self.SuspiciosPawn`)))
            (:`CastFailed`
              (`self.CheckThePawnIdentity`))))))))

(event `CheckThePawnIdentity`
  (bind _ashschar_base (cast `HSCharBase` (`self.SuspiciosPawn`))
    (:`then`
      (bind _bunitisteammate (message `/Game/WorkbenchModsSystem/Blueprints/Interfaces/BPI_WMS_UnitInterface.GetUnitIsTeammate` _ashschar_base))
      (if (!= _bunitisteammate (`self.bControlledPawnIsTeammate`))
        (`self.CheckIsUnitAlive` _ashschar_base
          (:`True`
            (add `HSCharBase.OnPreDead` _ashschar_base (`|CreateDelegate` :!event `OnTargetDead`))
            (if (`self.GetKnowAboutTarget_BB`)
              (`self.FF_Cooldown` 1.0
                (:`Completed`
                  (`self.TryToChangeTarget`)))
              (else
                (`self.SetTargetDependencies` (`self.SuspiciosPawn`)))))
          (:`false`
            (set `self.SuspiciosPawn` null :!label _label)))
        (else
          (goto _label))))
    (:`CastFailed`
      (goto _label))))

(event `OnPlayerDead`
  (`KismetSystemLibrary.Delay` 3.0)
  (`self.SetTarget_BB` null)
  (`self.SetTarget` null)
  (`self.SetKnowAboutTarget_BB` false))

(event `OnTargetDead`
  (params (Unit :type "HSCharBase Object Reference") (DamageCauser :type "Actor Object Reference") (PreviousState :type "EUnitState Enum" :default "CS_Idle"))
  (`KismetSystemLibrary.Delay` 0.5)
  (`self.SetTarget_BB` null)
  (`self.SetTarget` null)
  (`self.SetKnowAboutTarget_BB` false)
  (`self.CheckIfTeammatesNeedsHelp`))

(fn `CheckIfTeammatesNeedsHelp`
  (locals (ClosestDistance :type "Float (double-precision)" :default 115000.0) (TeammateToHelp :type "HSCharBase Object Reference"))
  (bind _outhits (`self.GetAllPawnsAround` (700.0 700.0 300.0)))
  (for _array_element _outhits
    (bind (_bblockinghit _binitialoverlap _time _distance _location _impactpoint _normal _impactnormal _physmat _hitactor) (`GameplayStatics.BreakHitResult` _array_element))
    (bind _ashschar_base (cast `HSCharBase` _hitactor))
    (bind _bunitisteammate (message `/Game/WorkbenchModsSystem/Blueprints/Interfaces/BPI_WMS_UnitInterface.GetUnitIsTeammate` _ashschar_base))
    (if (== _bunitisteammate (`self.bControlledPawnIsTeammate`))
      (if (< _distance (`local.ClosestDistance`))
        (`/Engine/EditorBlueprintResources/StandardMacros.IsValid` (`HSCharBase.GetTarget` _ashschar_base)
          (:`Is Valid`
            (set `local.ClosestDistance` _distance)
            (set `local.TeammateToHelp` _ashschar_base))))))
  (`/Engine/EditorBlueprintResources/StandardMacros.IsValid` (`local.TeammateToHelp`)
    (:`Is Valid`
      (bind _asbp_wms_simple_aicontroller (cast `/Game/WorkbenchModsSystem/Blueprints/AI/Controllers/BP_WMS_SimpleAIController` (`Pawn.GetController` (`local.TeammateToHelp`))))
      (bind _asactor (cast `Actor` (`self.GetTarget_BB` _asbp_wms_simple_aicontroller)))
      (`self.InstantlySeeTarget` _asactor))))

(fn `GetAllPawnsAround`
  (params (HalfSize :type "Vector Structure" :default (700.0 700.0 300.0)))
  (returns (OutHits :type "Array of HitResult Structure"))
  (bind _returnvalue (`self.K2_GetActorLocation` (`self.PossessedPawn`)))
  (bind _outhits (`KismetSystemLibrary.BoxTraceMultiForObjects` _returnvalue _returnvalue (`local.HalfSize`) (struct) (`|MakeArray` "ObjectTypeQuery3" :!type "EObjectTypeQuery Enum")))
  (return _outhits))

(fn `SetRandomTarget`
  (returns (bSuccess :type Boolean) (bTeammate :type Boolean))
  (locals (Enemies :type "Array of Pawn Object Reference"))
  (bind _enemies (`local.Enemies`))
  (bind _outhits (`self.GetAllPawnsAround` (52000.0 52000.0 5000.0)))
  (for _array_element _outhits
    (bind (_bblockinghit _binitialoverlap _time _distance _location _impactpoint _normal _impactnormal _physmat _hitactor) (`GameplayStatics.BreakHitResult` _array_element))
    (bind _ashschar_base (cast `HSCharBase` _hitactor)
      (:`then`
        (bind _bunitisteammate (message `/Game/WorkbenchModsSystem/Blueprints/Interfaces/BPI_WMS_UnitInterface.GetUnitIsTeammate` _ashschar_base))
        (if (!= _bunitisteammate (`self.bControlledPawnIsTeammate`))
          (`KismetArrayLibrary.Array_AddUnique` _enemies _ashschar_base)))
      (:`CastFailed`
        (bind _ashsplayer_avatar (cast `HSPlayerAvatar` _hitactor))
        (if (not (`self.bControlledPawnIsTeammate`))
          (`KismetArrayLibrary.Array_AddUnique` _enemies _ashsplayer_avatar)))))
  (if (`KismetArrayLibrary.Array_IsValidIndex` (`local.Enemies`))
    (`self.InstantlySeeTarget` (`KismetArrayLibrary.Array_Random` (`local.Enemies`)))
    (return true (`self.bControlledPawnIsTeammate`))
    (else
      (return false (`self.bControlledPawnIsTeammate`)))))

(fn `SetTargetDependencies`
  (params (InTarget :type "Pawn Object Reference"))
  (`self.SetTarget_BB` (`local.InTarget`))
  (`self.SetKnowAboutTarget_BB` true)
  (`self.SetTarget` (`local.InTarget`))
  (`self.CallOnAnyUnitSawTarget`)
  (bind _ashschar_base (cast `HSCharBase` (`self.PossessedPawn`)))
  (`HSCharBase.SetTarget` _ashschar_base (`local.InTarget`)))

(fn `TryToChangeTarget`
  (returns (bResult :type Boolean))
  (cast `Pawn` (`self.GetTarget_BB`))
  (if (< (`self.GetDistanceTo` (`self.SuspiciosPawn`) (`self.PossessedPawn`)) (`self.GetDistanceTo` (cast `Actor` (`self.GetTarget_BB`) :!pure true) (`self.PossessedPawn`)))
    (`self.SetTarget_BB` null)
    (`self.SetTarget` null)
    (`self.SetKnowAboutTarget_BB` false)
    (`self.SetTargetDependencies` (`self.SuspiciosPawn`))
    (return true)
    (else
      (return false))))

(fn `UserConstructionScript`
  (`parent.UserConstructionScript`))