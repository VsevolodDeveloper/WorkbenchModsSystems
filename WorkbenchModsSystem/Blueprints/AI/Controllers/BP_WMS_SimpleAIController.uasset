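; Base AI controller for Workbench Mods System enemy and teammate characters, managing target acquisition through Blackboard keys.
; On Blackboard setup, pawns implementing the enemy interface get sensing bound, the enemy director linked and optionally the player as initial target.
; Sighted pawns become the Target, and leaving a save zone re-initializes sensing.
; InstantlySeeTarget targets the hit causer, or the nearest eligible pawn filtered by team if that cast fails.
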(event `self.OnUsingBlackBoard`
  (params (BlackboardComp :type "BlackboardComponent Object Reference") (BlackboardAsset :type "BlackboardData Object Reference"))
  (`parent.OnUsingBlackBoard` BlackboardComp BlackboardAsset)
  (`self.SetCanWalk_BB` true)
  (if (`KismetSystemLibrary.DoesImplementInterface` (`self.PossessedPawn`) "/Game/WorkbenchModsSystem/Blueprints/Interfaces/BPI_WMS_EnemyInterface.BPI_WMS_EnemyInterface_C")
    (`self.Initialize`)))

(event `self.ReceivePossess`
  (params (PossessedPawn :type "Pawn Object Reference"))
  (`parent.ReceivePossess` PossessedPawn)
  (set `self.PossessedPawn` PossessedPawn))

(event `OnPlayerLeaveSaveZone`
  (params (LeftVolumeActor :type "Actor Object Reference"))
  (`self.IsPlayerInteractWithSaveZone` LeftVolumeActor
    (:`True`
      (`self.InitializeSensingComponent`))))

(event `OnPlayerEnteredSaveZone`
  (params (NewVolumeActor :type "Actor Object Reference")))

(event `OnSeeTarget`
  (params (Pawn :type "Pawn Object Reference"))
  (`self.SetTarget_BB` Pawn))

(fn `BindOnTargetInteractWithVolume`
  (bind _enemydirector (`self.EnemyDirector`)
    (:`then`
      (add `/Game/WorkbenchModsSystem/Blueprints/AI/BP_WMS_EnemyDirector.OnTargetEnteredNewVolume` _enemydirector (`|CreateDelegate` :!event `OnPlayerEnteredSaveZone`))
      (add `/Game/WorkbenchModsSystem/Blueprints/AI/BP_WMS_EnemyDirector.OnTargetLeaveVolume` _enemydirector (`|CreateDelegate` :!event `OnPlayerLeaveSaveZone`)))
    (:`else`)))

(fn `CallOnAnyUnitSawTarget`
  (bind _enemydirector (`self.EnemyDirector`)
    (:`then`
      (`/Game/WorkbenchModsSystem/Blueprints/AI/BP_WMS_EnemyDirector.OnAnyUnitSawTarget` _enemydirector (`self.PossessedPawn`)))
    (:`else`)))

(fn `GetKnowAboutTarget_BB`
  (returns (Value :type Boolean))
  (bind _returnvalue (`AIBlueprintHelperLibrary.GetBlackboard` null))
  (`/Engine/EditorBlueprintResources/StandardMacros.IsValid` _returnvalue
    (:`Is Valid`
      (return (`BlackboardComponent.GetValueAsBool` _returnvalue "KnowAboutTarget")))))

(fn `GetTarget_BB`
  (returns (Target :type "Object Object Reference"))
  (bind _returnvalue (`AIBlueprintHelperLibrary.GetBlackboard` null))
  (`/Engine/EditorBlueprintResources/StandardMacros.IsValid` _returnvalue
    (:`Is Valid`
      (return (`BlackboardComponent.GetValueAsObject` _returnvalue "Target")))))

(fn `Initialize`
  (`self.InitializeSensingComponent`)
  (`self.InitializeEnemyDirector`)
  (`self.BindOnTargetInteractWithVolume`)
  (`self.InitializePawn`))

(fn `InitializeEnemyDirector`
  (bind _returnvalue (`GameplayStatics.GetActorOfClass` "/Game/WorkbenchModsSystem/Blueprints/AI/BP_WMS_EnemyDirector.BP_WMS_EnemyDirector_C"))
  (set `self.EnemyDirector` _returnvalue))

(fn `InitializePawn`
  (bind _asbp_wms_simple_als_base_character (cast `/Game/WorkbenchModsSystem/Blueprints/Units/BaseUnits/BP_WMS_Simple_ALS_Base_Character` (`self.PossessedPawn`)))
  (bind _output_get (set `self.SimpleСharacter` _asbp_wms_simple_als_base_character))
  (set `self.bControlledPawnIsTeammate` (`/Game/WorkbenchModsSystem/Blueprints/Units/BaseUnits/BP_WMS_Simple_ALS_Base_Character.bTeammate` _output_get))
  (if (`HSCharBase.bSetPlayerAsTargetOnSpawn` (`self.SimpleСharacter`))
    (`self.OnSeeTarget` (`GameplayStatics.GetPlayerPawn` 0))))

(fn `InitializeSensingComponent`
  (`self.SensingComponent`
    (:`then`
      (add `PawnSensingComponent.OnSeePawn` (`self.SensingComponent`) (`|CreateDelegate` :!event `OnSeeTarget`)))
    (:`else`
      (bind _sensing_component (message `/Game/WorkbenchModsSystem/Blueprints/Interfaces/BPI_WMS_EnemyInterface.GetSensingComponent` (`self.PossessedPawn`)))
      (bind _output_get (set `self.SensingComponent` _sensing_component))
      (add `PawnSensingComponent.OnSeePawn` _output_get (`|CreateDelegate` :!event `OnSeeTarget`)))))

(fn `InstantlySeeTarget`
  (params (HitCauser :type "Actor Object Reference"))
  (locals (Pawns :type "Array of Pawn Object Reference") (SortedPawns :type "Array of Pawn Object Reference") (PawnToCheck :type "Pawn Object Reference"))
  (`/Engine/EditorBlueprintResources/StandardMacros.IsValid` HitCauser
    (:`Is Valid`
      (bind _aspawn (cast `Pawn` HitCauser)
        (:`then`
          (`self.OnSeeTarget` _aspawn))
        (:`CastFailed`
          (bind _outactors (`GameplayStatics.GetAllActorsOfClass` "/Script/Engine.Pawn")) ; Search for Hit Causer if it's nullptr
          (bind _output_get (set `local.Pawns` _outactors))
          (set `local.SortedPawns` _output_get)
          (for _array_element (`local.Pawns`)
            (set `local.PawnToCheck` _array_element)
            ;[1 1 1 1 28] Sort for nearest pawns that can be hit causer
            (`|ExecutionSequence`
              (:`then_0`
                (if (== (`local.PawnToCheck`) (`self.SimpleСharacter`))
                  (`KismetArrayLibrary.Array_RemoveItem` (`local.SortedPawns`) (`local.PawnToCheck`))))
              (:`then_1`
                (bind _asbp_wms_simple_als_base_character (cast `/Game/WorkbenchModsSystem/Blueprints/Units/BaseUnits/BP_WMS_Simple_ALS_Base_Character` (`local.PawnToCheck`)))
                (if (== (`/Game/WorkbenchModsSystem/Blueprints/Units/BaseUnits/BP_WMS_Simple_ALS_Base_Character.bTeammate` _asbp_wms_simple_als_base_character) (`self.bControlledPawnIsTeammate`))
                  (`KismetArrayLibrary.Array_RemoveItem` (`local.SortedPawns`) (`local.PawnToCheck`))))
              (:`then_2`
                (if (`self.bControlledPawnIsTeammate`)
                  (bind _ashsplayer_avatar (cast `HSPlayerAvatar` (`local.PawnToCheck`)))
                  (`KismetArrayLibrary.Array_RemoveItem` (`local.SortedPawns`) _ashsplayer_avatar)))
              (:`then_3`
                (bind _asspectator_pawn (cast `SpectatorPawn` (`local.PawnToCheck`)))
                (`KismetArrayLibrary.Array_RemoveItem` (`local.SortedPawns`) _asspectator_pawn))))
          (bind _aspawn_2 (cast `Pawn` (`.ReturnValue` (`GameplayStatics.FindNearestActor` (`self.K2_GetActorLocation` (`self.SimpleСharacter`)) (`local.SortedPawns`)))))
          (`self.OnSeeTarget` _aspawn_2))))))

(fn `SetCanWalk_BB`
  (params (bCanWalk :type Boolean))
  (`BlackboardComponent.SetValueAsBool` (`AIBlueprintHelperLibrary.GetBlackboard` null) "CanWalk" (`local.bCanWalk`)))

(fn `SetHandIsLost_BB`
  (params (bLost :type Boolean))
  (`/Engine/EditorBlueprintResources/StandardMacros.IsValid` (`AIBlueprintHelperLibrary.GetBlackboard` null)
    (:`Is Valid`
      (`BlackboardComponent.SetValueAsBool` (`AIBlueprintHelperLibrary.GetBlackboard` null) "HandIsLost" (`local.bLost`)))))

(fn `SetKnowAboutTarget_BB`
  (params (Value :type Boolean))
  (bind _returnvalue (`AIBlueprintHelperLibrary.GetBlackboard` null))
  (`/Engine/EditorBlueprintResources/StandardMacros.IsValid` _returnvalue
    (:`Is Valid`
      (`BlackboardComponent.SetValueAsBool` _returnvalue "KnowAboutTarget" (`local.Value`)))))

(fn `SetTarget_BB`
  (params (Target :type "Object Object Reference"))
  (bind _returnvalue (`AIBlueprintHelperLibrary.GetBlackboard` null))
  (`/Engine/EditorBlueprintResources/StandardMacros.IsValid` Target
    (:`Is Valid`
      (`/Engine/EditorBlueprintResources/StandardMacros.IsValid` _returnvalue
        (:`Is Valid`
          (`BlackboardComponent.SetValueAsObject` _returnvalue "Target" (`local.Target`)))))))

(fn `SetWanderingAreaFound_BB`
  (params (Value :type Boolean))
  (bind _returnvalue (`AIBlueprintHelperLibrary.GetBlackboard` null))
  (`/Engine/EditorBlueprintResources/StandardMacros.IsValid` _returnvalue
    (:`Is Valid`
      (`BlackboardComponent.SetValueAsBool` _returnvalue "WanderingAreaFound" Value))))

(fn `UserConstructionScript`
  (`parent.UserConstructionScript`))