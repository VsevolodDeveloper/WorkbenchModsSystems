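; BP_WMS_SimpleSaveZoneArea is a trigger-volume safe zone that hides the player from AI enemies while inside.
; Debounced overlaps with the player avatar raise enter/leave notifications and report the volume to BP_WMS_EnemyDirector.
; While occupied, a looping timer periodically sweeps all BP_WMS_SimpleAIController actors, clearing the target and awareness flag of any that know about their target.
; Leaving clears the timer.
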(event `OnSaveZoneEntered`
  (`self.OnSaveZoneAreaEntered`)
  (bind _returnvalue (`KismetSystemLibrary.K2_SetTimer` self "HidePlayerFromEnemies" 3.0 true))
  (set `self.CheckIsSeePlayerTimer` _returnvalue)
  (`self.UpdateCurrentVolume` self true))

(event `self.TriggerVolume.OnComponentBeginOverlap`
  (params (OverlappedComponent :type "PrimitiveComponent Object Reference") (OtherActor :type "Actor Object Reference") (OtherComp :type "PrimitiveComponent Object Reference") (OtherBodyIndex :type Integer) (bFromSweep :type Boolean) (SweepResult :type "HitResult Structure (by ref)"))
  (cast `HSPlayerAvatar` OtherActor)
  (`/Game/WorkbenchModsSystem/Blueprints/MacroLibrary/WMS_MacroLibrary.WMS_Cooldown` 0.1
    (:`Completed`
      (`self.OnSaveZoneEntered`))))

(event `self.TriggerVolume.OnComponentEndOverlap`
  (params (OverlappedComponent :type "PrimitiveComponent Object Reference") (OtherActor :type "Actor Object Reference") (OtherComp :type "PrimitiveComponent Object Reference") (OtherBodyIndex :type Integer))
  (cast `HSPlayerAvatar` OtherActor)
  (`/Game/WorkbenchModsSystem/Blueprints/MacroLibrary/WMS_MacroLibrary.WMS_Cooldown` 0.3
    (:`Completed`
      (`KismetSystemLibrary.K2_ClearAndInvalidateTimerHandle` (`self.CheckIsSeePlayerTimer`))
      (`self.OnSaveZoneAreaLeft`)
      (`self.UpdateCurrentVolume` self))))

(fn `HidePlayerFromEnemies`
  (bind _outactors (`GameplayStatics.GetAllActorsOfClass` "/Game/WorkbenchModsSystem/Blueprints/AI/Controllers/BP_WMS_SimpleAIController.BP_WMS_SimpleAIController_C"))
  (for _array_element _outactors
    (`/Engine/EditorBlueprintResources/StandardMacros.IsValid` _array_element
      (:`Is Valid`
        (if (`/Game/WorkbenchModsSystem/Blueprints/AI/Controllers/BP_WMS_SimpleAIController.GetKnowAboutTarget_BB` _array_element)
          (`HSEnemyAIController.SetTarget` _array_element null)
          (`/Game/WorkbenchModsSystem/Blueprints/AI/Controllers/BP_WMS_SimpleAIController.SetKnowAboutTarget_BB` _array_element false)))))
  (return))

(fn `UpdateCurrentVolume`
  (params (Volume :type "Actor Object Reference") (bEntered :type Boolean))
  (bind _returnvalue (`GameplayStatics.GetActorOfClass` "/Game/WorkbenchModsSystem/Blueprints/AI/BP_WMS_EnemyDirector.BP_WMS_EnemyDirector_C"))
  (`/Game/WorkbenchModsSystem/Blueprints/AI/BP_WMS_EnemyDirector.UpdateCurrentTargetVolume` _returnvalue (`local.Volume`) (`local.bEntered`)))

(fn `UserConstructionScript`)