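; Unit factory for AI units that spawns actors from named preset rows in a data table and reports each direct spawn's success.
; ALS characters receive HP, behavior, weapon and shield from the preset at spawn, while other classes spawn plain.
; A preset's extended-methods class, when set, is spawned as a helper actor that takes over creation.
; A custom-preset flag bypasses the table for CustomFactoryMethod, an empty hook here.
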(event `CallExtendedFactoryMethod`
  (params (FactoryMethodsLibrary :type "/Game/WorkbenchModsSystem/Blueprints/AI/UnitFactory/FactoryMethods/BP_WMS_FactoryMethodsLibrary Class Reference"))
  (bind _returnvalue (`|SpawnActorFromClass` FactoryMethodsLibrary (`KismetMathLibrary.MakeTransform` (0.0 0.0 0.0)) "AlwaysSpawn" "OverrideRootScale" null null))
  (bind _output_get (set `self.ExtendedFactoryLibrary` _returnvalue))
  (`/Engine/EditorBlueprintResources/StandardMacros.IsValid` _output_get
    (:`Is Valid`
      (set `/Game/WorkbenchModsSystem/Blueprints/AI/UnitFactory/FactoryMethods/BP_WMS_FactoryMethodsLibrary.Factory` self (`self.ExtendedFactoryLibrary`))
      (`/Game/WorkbenchModsSystem/Blueprints/AI/UnitFactory/FactoryMethods/BP_WMS_FactoryMethodsLibrary.Initialize` (`self.ExtendedFactoryLibrary`) (`self.UnitPreset`) (`self.SpawnTransform`) (`self.CollisionHandlingMethod`))
      (`/Game/WorkbenchModsSystem/Blueprints/AI/UnitFactory/FactoryMethods/BP_WMS_FactoryMethodsLibrary.FindAndCallExtendedMethod` (`self.ExtendedFactoryLibrary`)))
    (:`Is Not Valid`
      (`KismetSystemLibrary.PrintString` "Extended Method Library Is Null" true true (struct :`R` 1.0 :`G` 0.292559 :`A` 1.0)))))

(fn `CheckIsSpawnedUnitValid`
  (params (NewUnit :type "Actor Object Reference") (PresetName :type Name))
  (if (`KismetSystemLibrary.IsValid` NewUnit)
    (`self.OnUnitSpawned` (`local.NewUnit`) (`local.PresetName`) true)
    (else
      (`self.OnUnitSpawned` (`local.NewUnit`) (`local.PresetName`)))))

(fn `CustomFactoryMethod`
  (params (RowName :type Name) (SpawnTransform :type "Transform Structure"))
  (return))

(fn `ResetSpawnInformation`
  (params (RowName :type Name) (SpawnTransform :type "Transform Structure"))
  (set `self.UnitPreset` (struct))
  (set `self.SpawnTransform` SpawnTransform))

(fn `SpawnUnitFromPreset`
  (params (PresetName :type Name) (SpawnTransform :type "Transform Structure"))
  (bind ((`UnitClass_86_0B6F8D434BC27F54BA3219A0D11DAFA8` _unitclass) (`Weapon_11_9C47F970430A4FC7CCEE688AC44B1F53` _weapon) (`Shield_14_BD91D0D147A4CAB2B5C5C0A9DEAD6C99` _shield) (`WeaponAmplificators_58_B5A6A8C8473F585D79DA019D6EF63785` _weaponamplificators) (`HeadHP_37_7430857740F0C94BEDE3B3B1569A604F` _headhp) (`BodyHP_38_9601A4874A60EBAF17CD8392039EFB5B` _bodyhp) (`DefaultBehaviorPattern_30_958656144773A694EA98548B68E7A5A4` _defaultbehaviorpattern) (`RunBehaviorTree_83_E68AB0074E71D9391EC2729AC177F9E4` _runbehaviortree)) (break `/Game/WorkbenchModsSystem/Blueprints/AI/UnitFactory/F_WMS_UnitPreset` (`self.UnitPreset`)))
  (`self.ResetSpawnInformation` PresetName SpawnTransform)
  (if (not (`self.CustomUnitPresetStructure`))
    (bind _returnvalue (`|GetDataTableRow` (`self.UnitPresetsData`) (`local.PresetName`))
      (:`then`
        (set `self.UnitPreset` _returnvalue)
        (if (not (`KismetSystemLibrary.IsValidClass` (`.ExtendedFactoryMethodsLibrary_85_EB14BDB64BBBC470D79049A22DA6DF7C` (break `/Game/WorkbenchModsSystem/Blueprints/AI/UnitFactory/F_WMS_UnitPreset` (`self.UnitPreset`)))))
          (bind _asals_base_character (castclass `/Game/Blueprints/Units/ALS_BaseCharacter` _unitclass)
            (:`then`
              (bind _returnvalue_2 (`|SpawnActorFromClass` :`Class` _asals_base_character :`SpawnTransform` (`local.SpawnTransform`) :`CollisionHandlingOverride` (`self.CollisionHandlingMethod`) :`TransformScaleMethod` "OverrideRootScale" :`HeadInitialHP` _headhp :`BodyInitialHP` _bodyhp :`bRunBehaviourTree` _runbehaviortree :`DefaultBehavior` _defaultbehaviorpattern :`bPlayIntroMontage` true :`WeaponClass` _weapon :`ShieldClass` _shield :`StoredWeaponAmplificator` null :`Instigator` null))
              (`self.CheckIsSpawnedUnitValid` _returnvalue_2 (`local.PresetName`)))
            (:`CastFailed`
              (bind _returnvalue_3 (`|SpawnActorFromClass` (`.UnitClass_86_0B6F8D434BC27F54BA3219A0D11DAFA8` (break `/Game/WorkbenchModsSystem/Blueprints/AI/UnitFactory/F_WMS_UnitPreset` (`self.UnitPreset`))) (`local.SpawnTransform`) (`self.CollisionHandlingMethod`) "OverrideRootScale" null null))
              (`self.CheckIsSpawnedUnitValid` _returnvalue_3 (`local.PresetName`))))
          (else
            (`self.CallExtendedFactoryMethod` (`.ExtendedFactoryMethodsLibrary_85_EB14BDB64BBBC470D79049A22DA6DF7C` (break `/Game/WorkbenchModsSystem/Blueprints/AI/UnitFactory/F_WMS_UnitPreset` (`self.UnitPreset`)))))))
      (:`RowNotFound`
        (`KismetSystemLibrary.PrintString` "UnitPreset Not Found" true true (struct :`R` 1.0 :`G` 0.046319 :`A` 1.0))
        (return)))
    (else
      (`self.CustomFactoryMethod` (`local.PresetName`) (`self.SpawnTransform`)))))

(fn `UserConstructionScript`
  (`parent.UserConstructionScript`))