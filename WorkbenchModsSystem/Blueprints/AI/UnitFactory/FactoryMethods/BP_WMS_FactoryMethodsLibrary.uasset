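; Short-lived actor that hosts extended factory methods for spawning units from a unit preset in the WMS unit factory.
; Initialize caches the preset, spawn transform, collision handling and the preset's extended factory config.
; FindAndCallExtendedMethod invokes the method named by that config through a 0.1-second timer by function name, printing an error if the config is invalid.
; CheckSpawnedUnit passes the new unit to the factory for validation, then destroys this actor.
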(event `FindAndCallExtendedMethod`
  (`/Engine/EditorBlueprintResources/StandardMacros.IsValid` (`self.ExtendedFactoryConfig`)
    (:`Is Valid`
      (`KismetSystemLibrary.K2_SetTimer` self (`/Game/WorkbenchModsSystem/Blueprints/AI/UnitFactory/FactoryMethods/BP_WMS_UnitProperties.GetFactoryMethodName` (`self.ExtendedFactoryConfig`)) 0.1))
    (:`Is Not Valid`
      (`KismetSystemLibrary.PrintString` "Factory Data Asset Is Null" true true (struct :`R` 1.0 :`A` 1.0)))))

(fn `CheckSpawnedUnit`
  (params (NewUnit :type "Actor Object Reference"))
  (`/Game/WorkbenchModsSystem/Blueprints/AI/UnitFactory/BP_WMS_UnitFactory.CheckIsSpawnedUnitValid` (`self.GetFactory`) (`local.NewUnit`) (`.PresetName_61_1B3669E4402CD88972C70D9396EB9BBE` (break `/Game/WorkbenchModsSystem/Blueprints/AI/UnitFactory/F_WMS_UnitPreset` (`self.UnitPreset`))))
  (`self.K2_DestroyActor`))

(fn `GetFactory`
  (returns (Factory :type "/Game/WorkbenchModsSystem/Blueprints/AI/UnitFactory/BP_WMS_UnitFactory Object Reference"))
  (return (`self.Factory`)))

(fn `Initialize`
  (params (UnitPreset :type "/Game/WorkbenchModsSystem/Blueprints/AI/UnitFactory/F_WMS_UnitPreset Structure") (SpawnTransform :type "Transform Structure") (CollisionHandling :type "ESpawnActorCollisionHandlingMethod Enum" :default "Undefined"))
  (set `self.UnitPreset` UnitPreset)
  (set `self.SpawnTransform` SpawnTransform)
  (set `self.SpawnCollisionHandling` CollisionHandling)
  (set `self.ExtendedFactoryConfig` (`.ExtendedFactoryConfig_84_9D75FA7B4DF2AA9E1ABE2D8446961E63` (break `/Game/WorkbenchModsSystem/Blueprints/AI/UnitFactory/F_WMS_UnitPreset` (`self.UnitPreset`)))))

(fn `UserConstructionScript`)