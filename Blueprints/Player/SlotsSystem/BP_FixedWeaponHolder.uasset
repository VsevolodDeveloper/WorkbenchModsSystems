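; BP_FixedWeaponHolder is a holder in the player slots system that refuses actors carrying certain gameplay tags.
; SetTags replaces the stored GameplayTags, which act as an exclusion list.
; IsActorAcceptable rejects an actor if its tags match any of these, using non-exact matching so child tags also count, and otherwise defers to the parent's check.
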(event `/Game/WorkbenchModsSystem/Blueprints/Interfaces/BPI_WMS_SlotInterface.SetTags`
  (params (Tags :type "GameplayTagContainer Structure"))
  (set `self.GameplayTags` Tags))

(fn `IsActorAcceptable`
  (params (ActorToHold :type "Actor Object Reference"))
  (returns (ReturnValue :type Boolean))
  (bind _outcontainer (`HSCommonFunctionLibrary.GetActorGameplayTags` ActorToHold))
  (if (`BlueprintGameplayTagLibrary.HasAnyTags` _outcontainer (`self.GameplayTags`))
    (return false)
    (else
      (bind _returnvalue (`parent.IsActorAcceptable` (`local.ActorToHold`)))
      (return _returnvalue))))

(fn `UserConstructionScript`
  (`parent.UserConstructionScript`))