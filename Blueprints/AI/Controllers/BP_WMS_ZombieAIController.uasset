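; AI controller for zombies that acquires a target by sight or on being hit, and drops it when the player dies.
; Seeing a player avatar sets the target and blackboard awareness, broadcasts the sighting and unbinds a see-pawn handler from the sensing component.
; Initialize binds to the possessed ALS character's hit event so a zombie without a valid target instantly sees the hit causer.
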(event `self.OnSeeTarget`
  (params (Pawn :type "Pawn Object Reference"))
  (`parent.OnSeeTarget` Pawn)
  (bind _ashsplayer_avatar (cast `HSPlayerAvatar` Pawn))
  (add `HSVRCharacter.OnDead` _ashsplayer_avatar (delegate `OnPlayerDead`))
  (`self.SetKnowAboutTarget_BB` true)
  (`self.SetTarget` Pawn)
  (`self.CallOnAnyUnitSawTarget`)
  (remove `PawnSensingComponent.OnSeePawn` (`self.SensingComponent`) (`|CreateDelegate` :!event `OnSeeTarget`)))

(event `OnPlayerDead`
  (`self.SetTarget` null)
  (`self.SetKnowAboutTarget_BB` false))

(event `OnEnemyHit`
  (params (HitCauser :type "Actor Object Reference"))
  (`/Engine/EditorBlueprintResources/StandardMacros.IsValid` (`self.GetTarget_BB`)
    (:`Is Not Valid`
      (`self.InstantlySeeTarget` HitCauser))))

(fn `Initialize`
  (`parent.Initialize`)
  (bind _asbp_wms_simple_als_base_character (cast `/Game/WorkbenchModsSystem/Blueprints/Units/BaseUnits/BP_WMS_Simple_ALS_Base_Character` (`self.PossessedPawn`)))
  (add `/Game/WorkbenchModsSystem/Blueprints/Units/BaseUnits/BP_WMS_Simple_ALS_Base_Character.OnEnemyHit` _asbp_wms_simple_als_base_character (`|CreateDelegate` :!event `OnEnemyHit`)))

(fn `UserConstructionScript`)