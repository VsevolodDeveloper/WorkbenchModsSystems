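; Unit factory method Blueprint that spawns WMS Simple ALS base characters from a unit preset.
; SpawnBaseCharacter casts the extended factory config and preset class, stopping if either fails, then passes per-body-part HP, behavior, weapon, shield and a random weapon amplificator into the spawn.
; Chopping and firearm damage come from the config, while blunt damage gets a default-built struct.
; The intro montage is always enabled, and the result goes to CheckSpawnedUnit.
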(fn `SpawnBaseCharacter`
  (bind ((`UnitClass_86_0B6F8D434BC27F54BA3219A0D11DAFA8` _unitclass) (`Weapon_11_9C47F970430A4FC7CCEE688AC44B1F53` _weapon) (`Shield_14_BD91D0D147A4CAB2B5C5C0A9DEAD6C99` _shield) (`WeaponAmplificators_58_B5A6A8C8473F585D79DA019D6EF63785` _weaponamplificators) (`HeadHP_37_7430857740F0C94BEDE3B3B1569A604F` _headhp) (`BodyHP_38_9601A4874A60EBAF17CD8392039EFB5B` _bodyhp) (`DefaultBehaviorPattern_30_958656144773A694EA98548B68E7A5A4` _defaultbehaviorpattern) (`RunBehaviorTree_83_E68AB0074E71D9391EC2729AC177F9E4` _runbehaviortree)) (break `/Game/WorkbenchModsSystem/Blueprints/AI/UnitFactory/F_WMS_UnitPreset` (`self.UnitPreset`)))
  (bind _asup_simple_als_base_character (cast `/Game/WorkbenchModsSystem/Blueprints/AI/UnitFactory/FactoryMethods/WMS_UnitsMethods/UP_Simple_ALS_Base_Character` (`self.ExtendedFactoryConfig`)))
  (bind _asbp_wms_simple_als_base_character (castclass `/Game/WorkbenchModsSystem/Blueprints/Units/BaseUnits/BP_WMS_Simple_ALS_Base_Character` _unitclass))
  (bind _returnvalue (`|SpawnActorFromClass` :`Class` _asbp_wms_simple_als_base_character :`SpawnTransform` (`self.SpawnTransform`) :`CollisionHandlingOverride` (`self.SpawnCollisionHandling`) :`TransformScaleMethod` "OverrideRootScale" :`DamageFromChoppingWeapons` (`/Game/WorkbenchModsSystem/Blueprints/AI/UnitFactory/FactoryMethods/WMS_UnitsMethods/UP_Simple_ALS_Base_Character.DamageFromChoppingWeapons` _asup_simple_als_base_character) :`DamageFromBluntWeapons` (make `/Game/WorkbenchModsSystem/Blueprints/Units/DamageData/F_WMS_DamageByBodyParts` _) :`DamageFromFirearms` (`/Game/WorkbenchModsSystem/Blueprints/AI/UnitFactory/FactoryMethods/WMS_UnitsMethods/UP_Simple_ALS_Base_Character.DamageFromFirearms` _asup_simple_als_base_character) :`HeadInitialHP` _headhp :`BodyInitialHP` _bodyhp :`bRunBehaviourTree` _runbehaviortree :`DefaultBehavior` _defaultbehaviorpattern :`bPlayIntroMontage` true :`WeaponClass` _weapon :`ShieldClass` _shield :`StoredWeaponAmplificator` (`KismetArrayLibrary.Array_Random` _weaponamplificators) :`Instigator` null))
  (`self.CheckSpawnedUnit` _returnvalue))

(fn `UserConstructionScript`
  (`parent.UserConstructionScript`))