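; Base class for enemy units that fight with a two-handed firearm, spawned into the right hand on BeginPlay.
; A looping timer checks ammo in combat and triggers a montage-driven reload that manages magazine and left-hand constraint.
; Each shot updates the target, applies physics recoil to arm bones, crossfades near/far sounds and randomizes aim.
; Death or arm dismemberment drops the gun and flags the AI; Initialize also overrides player bullet-damage multipliers.
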(event `self.ReceiveBeginPlay`
  (`parent.ReceiveBeginPlay`)
  (`self.SpawnFirearm`)
  (add `self.OnRagdollEnded` (delegate `OnRagdollEndedEvent`))
  (`KismetSystemLibrary.K2_SetTimerDelegate` (delegate `CheckAmmoAmount`) 0.1 true)
  (`KismetSystemLibrary.Delay` 0.1) ; PostInitialize
  (bind _firearm (`self.Firearm`)
    (:`then`
      (add `HSGunBarrelComponent.OnShot` (`/Game/WorkbenchModsSystem/Blueprints/Units/Firearms/BP_WMS_EnemyFirearmBase.Barrel` _firearm) (`|CreateDelegate` :!event `OnShot`))
      (add `self.OnPreDead` (`|CreateDelegate` :!event `OnDead`)))
    (:`else`)))

(event `OnRagdollEndedEvent` :!signature `self.OnRagdollEnded`
  (params (ToFoot :type Boolean))
  (if ToFoot
    (`self.Set ALS_Stance Event` "NewEnumerator0")))

(event `CheckAmmoAmount`
  (if (`|EnumEquality` (`self.GetUnitState`) "CS_Combat")
    (bind _firearm (`self.Firearm`)
      (:`then`
        (bind _returnvalue (`/Game/WorkbenchModsSystem/Blueprints/Units/Firearms/BP_WMS_EnemyFirearmBase.AmmoIsOut` _firearm))
        (if _returnvalue
          (`/Engine/EditorBlueprintResources/StandardMacros.DoOnce` _returnvalue :!label _label
            (:`Completed`
              (`self.ReloadTheWeapon`)))
          (else
            (goto _label :!via `Reset`))))
      (:`else`))))

(event `self.UnitInjuries.OnPostDismemberment`
  (params (BodyPart :type "EUnitBodyPart Enum" :default "None") (bInitialPart :type Boolean) (BodyPartActor :type "HSSlicedUnitBodyPart Object Reference") (DismembermentRule :type "BodyPartDismembermentRule Object Reference"))
  (if (or (not (`HSUnitInjuriesComponent.IsBodyPartExists` (`self.UnitInjuries`) "forearm_l" false)) (not (`HSUnitInjuriesComponent.IsBodyPartExists` (`self.UnitInjuries`) "shoulder_l" false)) (not (`HSUnitInjuriesComponent.IsBodyPartExists` (`self.UnitInjuries`) "forearm_r" false)) (not (`HSUnitInjuriesComponent.IsBodyPartExists` (`self.UnitInjuries`) "shoulder_r" false)))
    (`self.DropFirearm`)))

(event `ReloadTheWeapon`
  (bind _firearm (`self.Firearm`)
    (:`then`
      (`/Game/WorkbenchModsSystem/Blueprints/Units/Firearms/BP_WMS_EnemyFirearmBase.StartToReload` _firearm)
      (`/Game/WorkbenchModsSystem/Blueprints/Units/Firearms/BP_WMS_EnemyFirearmBase.UnlinkHands` (`self.Firearm`) (`self.LeftHandsConstraint`))
      (`|PlayMontage` (`self.Mesh`) (`/Game/WorkbenchModsSystem/Blueprints/Units/Firearms/BP_WMS_EnemyFirearmBase.ReloadMontage` _firearm)
        (:`then`
          (bind _firearm_2 (`self.Firearm`)
            (:`then`
              (`/Game/WorkbenchModsSystem/Blueprints/Units/Firearms/BP_WMS_EnemyFirearmBase.SpawnMagazine` _firearm_2 (`self.Mesh`)))
            (:`else`)))
        (:`OnCompleted`
          (bind _firearm_3 (`self.Firearm`)
            (:`then`
              (`/Game/WorkbenchModsSystem/Blueprints/Units/Firearms/BP_WMS_EnemyFirearmBase.FinishReload` _firearm_3)
              (`/Game/WorkbenchModsSystem/Blueprints/Units/Firearms/BP_WMS_EnemyFirearmBase.LinkHands` (`self.Firearm`) (`self.LeftHandsConstraint`) :!label _label_2))
            (:`else`)))
        (:`OnInterrupted`
          (bind _firearm_4 (`self.Firearm`)
            (:`then`
              (`/Game/WorkbenchModsSystem/Blueprints/Units/Firearms/BP_WMS_EnemyFirearmBase.SpawnMagazine` _firearm_4 (`self.Mesh`))
              (`/Game/WorkbenchModsSystem/Blueprints/Units/Firearms/BP_WMS_EnemyFirearmBase.AttachMagazine` _firearm_4)
              (`/Game/WorkbenchModsSystem/Blueprints/Units/Firearms/BP_WMS_EnemyFirearmBase.FinishReload` _firearm_4)
              (goto _label_2))
            (:`else`)))
        (:`OnNotifyBegin`
          (bind _firearm_5 (`self.Firearm`)
            (:`then`
              (`/Game/WorkbenchModsSystem/Blueprints/Units/Firearms/BP_WMS_EnemyFirearmBase.AttachMagazine` _firearm_5))
            (:`else`)))))
    (:`else`)))

(event `OnShot`
  (params (Barrel :type "HSGunBarrelComponent Object Reference") (Cartridge :type "HSFirearmCartridgeInterface Interface (by ref)") (Bullets :type "Array of Actor Object Reference (by ref)"))
  (`self.UpdateWeaponTarget`)
  (`self.ApplyRecoilFromFirearm`)
  (`self.PlayShotSoundsFromFirearm`)
  (`self.SetRandomAimDeviation`))

(event `OnDead` :!signature `self.OnPreDead`
  (params (Unit :type "HSCharBase Object Reference") (DamageCauser :type "Actor Object Reference") (PreviousState :type "EUnitState Enum" :default "CS_Idle"))
  (`self.DropFirearm`))

(fn `ApplyRecoilFromFirearm`
  (`self.Firearm`
    (:`then`
      (`PrimitiveComponent.AddImpulse` (`self.Mesh`) (`KismetMathLibrary.MakeVector` 0.0 0.0 (`/Game/WorkbenchModsSystem/Blueprints/Units/Firearms/BP_WMS_EnemyFirearmBase.RecoilImpulse` (`self.Firearm`))) "lowerarm_r" true)
      (if (`/Game/WorkbenchModsSystem/Blueprints/Units/Firearms/BP_WMS_EnemyFirearmBase.bConstrainedMode` (`self.Firearm`))
        (`PrimitiveComponent.AddImpulse` (`self.Mesh`) (`KismetMathLibrary.MakeVector` 0.0 0.0 (`/Game/WorkbenchModsSystem/Blueprints/Units/Firearms/BP_WMS_EnemyFirearmBase.RecoilImpulse` (`self.Firearm`))) "lowerarm_l" true)))
    (:`else`)))

(fn `DropFirearm`
  (bind _firearm (`self.Firearm`)
    (:`then`
      (`self.SetLifeSpan` _firearm 5.0)
      (bind _firearm_2 (`self.Firearm`)
        (:`then`
          (`self.K2_DetachFromActor` _firearm_2 "KeepWorld" "KeepWorld" "KeepRelative")
          (`self.SetActorEnableCollision` (`self.Firearm`) true)
          (bind _firearm_3 (`self.Firearm`)
            (:`then`
              (bind _meshcomp (`HSWeaponBase.MeshComp` _firearm_3))
              (`PrimitiveComponent.SetCollisionEnabled` _meshcomp "QueryAndPhysics")
              (`PrimitiveComponent.SetCollisionObjectType` _meshcomp "ECC_PhysicsBody")
              (`PrimitiveComponent.SetSimulatePhysics` _meshcomp true)
              (`PrimitiveComponent.SetEnableGravity` _meshcomp true)
              (bind _asbp_wms_simple_aicontroller (cast `/Game/WorkbenchModsSystem/Blueprints/AI/Controllers/BP_WMS_SimpleAIController` (`AIBlueprintHelperLibrary.GetAIController` self)))
              (`/Game/WorkbenchModsSystem/Blueprints/AI/Controllers/BP_WMS_SimpleAIController.SetHandIsLost_BB` _asbp_wms_simple_aicontroller true)
              (set `self.Firearm` null))
            (:`else`)))
        (:`else`)))
    (:`else`)))

(fn `Initialize`
  (`parent.Initialize`)
  (`/Engine/EditorBlueprintResources/StandardMacros.IsValid` (`HSPlayerFunctionLibrary.GetPlayerAvatar`)
    (:`Is Valid`
      ;[1 0.05208 0.05208] A little hack, so that the player does not die instantly
      (set `HSPlayerAvatar.BulletBodyShotDamageMultiplier` 1.0 (`HSPlayerFunctionLibrary.GetPlayerAvatar`))
      (set `HSPlayerAvatar.BulletHeadShotDamageMultiplier` 1.0 (`HSPlayerFunctionLibrary.GetPlayerAvatar`)))))

(fn `PlayShotSoundsFromFirearm`
  (bind _firearm (`self.Firearm`))
  (bind _farshotdistancerange (`/Game/WorkbenchModsSystem/Blueprints/Units/Firearms/BP_WMS_EnemyFirearmBase.FarShotDistanceRange` _firearm))
  (bind _returnvalue (- (`self.GetDistanceTo` (`GameplayStatics.GetPlayerPawn` 0) self) (`/Game/WorkbenchModsSystem/Blueprints/Units/Firearms/BP_WMS_EnemyFirearmBase.FarShotDistance` _firearm)))
  (`self.Firearm`
    (:`then`
      (if (`/Game/WorkbenchModsSystem/Blueprints/Units/Firearms/BP_WMS_EnemyFirearmBase.bSetShotSoundsByDistance` (`self.Firearm`))
        (`/Engine/EditorBlueprintResources/StandardMacros.IsValid` (`self.GetTarget`)
          (:`Is Valid`
            (`GameplayStatics.PlaySoundAtLocation` (`/Game/WorkbenchModsSystem/Blueprints/Units/Firearms/BP_WMS_EnemyFirearmBase.FarShotSound` (`self.Firearm`)) (`self.K2_GetActorLocation`) (struct) (`KismetMathLibrary.MapRangeClamped` _returnvalue 0.0 _farshotdistancerange 0.0 1.0) 1.0 0.0 null null null)
            (`GameplayStatics.PlaySoundAtLocation` (`/Game/WorkbenchModsSystem/Blueprints/Units/Firearms/BP_WMS_EnemyFirearmBase.CloseShotSound` (`self.Firearm`)) (`self.K2_GetActorLocation`) (struct) (`KismetMathLibrary.MapRangeClamped` _returnvalue _farshotdistancerange 0.0 0.0 1.0) 1.0 0.0 null null null)))))
    (:`else`)))

(fn `SpawnFirearm`
  (`self.DropWeapon`)
  (if (`KismetSystemLibrary.IsValidClass` (`self.FirearmClass`))
    (bind _returnvalue (`|SpawnActorFromClass` (`self.FirearmClass`) (`KismetMathLibrary.MakeTransform` (0.0 0.0 0.0)) "AlwaysSpawn" "OverrideRootScale" null null))
    (bind _output_get (set `self.Firearm` _returnvalue))
    (`self.K2_AttachToComponent` _output_get (`self.Mesh`) "socket_hand_r_sword" "SnapToTarget" "SnapToTarget" "KeepRelative" true)
    (`/Game/WorkbenchModsSystem/Blueprints/Units/Firearms/BP_WMS_EnemyFirearmBase.AddWeaponOffset` (`self.Firearm`))
    (`/Game/WorkbenchModsSystem/Blueprints/Units/Firearms/BP_WMS_EnemyFirearmBase.SetTwoHandedMode` (`self.Firearm`) (`self.Mesh`) (`self.LeftHandsConstraint`))))

(fn `UpdateWeaponTarget`
  (`self.Firearm`
    (:`then`
      (set `/Game/WorkbenchModsSystem/Blueprints/Units/Firearms/BP_WMS_EnemyFirearmBase.Target` (`self.GetTarget`) (`self.Firearm`)))
    (:`else`)))

(fn `UserConstructionScript`
  (`parent.UserConstructionScript`))