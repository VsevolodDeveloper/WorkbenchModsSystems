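; Base Blueprint for a simplified enemy shotgun with foreend, magazine gate, magazine and barrel components.
; AttachMagazine spawns ammo and mounts it in the gate, which animates open and pushes dismounted rounds into the magazine.
; The foreend chambers non-shell cartridges through callbacks and events and never reports itself locked.
; Shot skips foreend cycling, popping a cartridge straight from the magazine into the barrel and firing unless reloading.
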(event `self.ReceiveBeginPlay`
  ;[1 1 1] Initialization
  (`parent.ReceiveBeginPlay`)
  (set `HSPumpShotgunForendComponent.IsLockedCallback` (`|CreateDelegate` :!event `IsForeendLocked`) (`self.Foreend`))
  (set `HSFirearmBoltComponentBase.GetAmmoCallback` (`|CreateDelegate` :!event `LoadAmmo`) (`self.Foreend`))
  (set `MountSlotComponent.CanMountCallback` (`|CreateDelegate` :!event `CanLoadCartridgeToMagazine`) (`self.MagazineGate`)))

(event `self.Foreend.OnMovedToInitialPosition`
  (params (Bolt :type "HSFirearmBoltComponentBase Object Reference") (Ammo :type "Actor Object Reference"))
  ;[1 1 1] Foreend (bolt) events
  (bind _ashsfirearm_cartridge_interface (cast `HSFirearmCartridgeInterface` Ammo))
  (if (not (`HSFirearmCartridgeInterface.IsShell` _ashsfirearm_cartridge_interface))
    (`HSGunBarrelComponent.SetCartridge` (`self.BarrelComponent`) _ashsfirearm_cartridge_interface)))

(event `self.Foreend.OnMovedFromInitialPosition`
  (params (Bolt :type "HSFirearmBoltComponentBase Object Reference") (Ammo :type "Actor Object Reference"))
  ;[1 1 1] Foreend (bolt) events
  (`HSGunBarrelComponent.RemoveCartridge` (`self.BarrelComponent`)))

(event `self.BarrelComponent.OnShot`
  (params (Barrel :type "HSGunBarrelComponent Object Reference") (Cartridge :type "HSFirearmCartridgeInterface Interface (by ref)") (Bullets :type "Array of Actor Object Reference (by ref)"))
  ;[1 0.4094 0.05208] Shot!
  (`HSPumpShotgunForendComponent.Unlock` (`self.Foreend`)) ; Automatically unlock the foreend
)

(event `self.MagazineGate.OnBeginMounting`
  (params (Slot :type "MountSlotComponent Object Reference") (MountableActor :type "Actor Object Reference") (MountablePrimitive :type "PrimitiveComponent Object Reference") (MountableComponent :type "MountableComponent Object Reference"))
  ;[1 1 1] Play simple gate open animation
  (bind (_direction _time) (`Timeline|OpenGate` :!via `PlayFromStart`)
    (:`Update`
      (`HSSupportingLeverComponent.SetRotationAtTime` (`self.Gate`) _time))))

(event `self.MagazineGate.OnComponentDismounted`
  (params (Slot :type "MountSlotComponent Object Reference") (MountedActor :type "Actor Object Reference") (MountedPrimitive :type "PrimitiveComponent Object Reference") (MountableComponent :type "MountableComponent Object Reference"))
  ;[0.3873 0.818 1] Automatically load the cartridge to the magazine after mounting to the slot
  ; The slot "GateMode" is set to true
  (`HSActorsStackComponent.Push` (`self.MagazineComponent`) MountedActor))

(fn `AttachMagazine`
  (locals (Ammo :type "HSFirearmCartridgeBase Object Reference"))
  (bind _returnvalue (`|SpawnActorFromClass` (`self.ShotgunAmmo`) (`SceneComponent.GetSocketTransform` (`self.MeshComp`) "socket_bow" "RTS_World") "AlwaysSpawn" "OverrideRootScale" null null))
  (bind _output_get (set `local.Ammo` _returnvalue))
  (`/Engine/EditorBlueprintResources/StandardMacros.IsValid` _output_get
    (:`Is Valid`
      (bind _returnvalue_2 (`self.GetComponentByClass` _output_get "/Script/ElasticVR.MountableComponent"))
      (`/Engine/EditorBlueprintResources/StandardMacros.IsValid` _returnvalue_2
        (:`Is Valid`
          (`MountSlotComponent.MountComponent` (`self.MagazineGate`) _returnvalue_2 true false))))))

(fn `CanLoadCartridgeToMagazine`
  (params (Slot :type "MountSlotComponent Object Reference"))
  (returns (ReturnValue :type Boolean))
  (return (not (`HSActorsStackComponent.IsFull` (`self.MagazineComponent`)))))

(fn `IsForeendLocked`
  (returns (ReturnValue :type Boolean))
  (return false))

(fn `LoadAmmo`
  (returns (ReturnValue :type "Actor Object Reference"))
  (bind _returnvalue (`HSActorsStackComponent.Pop` (`self.MagazineComponent`)))
  (return _returnvalue))

(fn `Shot`
  (if (not (`self.bReloading`))
    (bind _returnvalue (`HSActorsStackComponent.Pop` (`self.MagazineComponent`)))
    (bind _ashsfirearm_cartridge_interface (cast `HSFirearmCartridgeInterface` _returnvalue))
    (`HSGunBarrelComponent.SetCartridge` (`self.BarrelComponent`) _ashsfirearm_cartridge_interface)
    (`HSGunBarrelComponent.Shot` (`self.BarrelComponent`))))

(fn `TurnForeendSafetyOff`
  (set `self.bForeendSafetyOn` false))

(fn `TurnForeendSafetyOn`
  (set `self.bForeendSafetyOn` true))

(fn `UserConstructionScript`)